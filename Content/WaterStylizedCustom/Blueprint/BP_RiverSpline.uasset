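; BP_RiverSpline is a spline-driven actor that builds a river surface along an editable path.
; The Construction Script adds one spline mesh component per segment, applies RiverMaterial and matches each segment's start and end to the spline's local positions and tangents.
; Per-point spline scale multiplied by RiverWidth sets each segment's end scales, so the river's cross-section can vary along its course.
; The event graph holds no runtime logic.
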(fn `UserConstructionScript`
  (bind _spline (`self.Spline`))
  (bind _spline_2 (`self.Spline`))
  (bind _river_width (`self.River Width`))
  (bind _river_width_2 (`self.River Width`))
  (for _index (range (+ (- (`SplineComponent.GetNumberOfSplinePoints` (`self.Spline`)) 2) 1))
    (bind _returnvalue (`AddComponent|NODE_AddSplineMeshComponent-0`))
    (`PrimitiveComponent.SetMaterial` _returnvalue 0 (`self.River Material`))
    (bind (_returnvalue_x _returnvalue_y) (`KismetMathLibrary.BreakVector` (`SplineComponent.GetScaleAtSplinePoint` _spline_2 _index)))
    (`SplineMeshComponent.SetStartScale` _returnvalue (`KismetMathLibrary.MakeVector2D` (* _returnvalue_x _river_width_2) (* _river_width_2 _returnvalue_y)) true)
    (bind (_returnvalue_x_2 _returnvalue_y_2) (`KismetMathLibrary.BreakVector` (`SplineComponent.GetScaleAtSplinePoint` _spline_2 (+ _index 1))))
    (`SplineMeshComponent.SetEndScale` _returnvalue (`KismetMathLibrary.MakeVector2D` (* _returnvalue_x_2 _river_width) (* _river_width _returnvalue_y_2)) true)
    (`SceneComponent.K2_AttachToComponent` _returnvalue null "None" "KeepRelative" "KeepRelative" "KeepRelative" true)
    (bind (_location _tangent) (`SplineComponent.GetLocationAndTangentAtSplinePoint` _spline _index "Local"))
    (bind (_location_2 _tangent_2) (`SplineComponent.GetLocationAndTangentAtSplinePoint` _spline (+ _index 1) "Local"))
    (`SplineMeshComponent.SetStartAndEnd` _returnvalue _location _tangent _location_2 _tangent_2 true)))