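; BP_TimeSkipVFXController is meant to drive a time-skip effect through the PostProcessGlobal material parameter collection, but no event runs its logic.
; At slowed global time dilation, the graph writes camera forward into PlayerPosition and increments EndOfTimeOffset, though a zero multiplier on SpaceSpeed leaves it unchanged.
; Otherwise, it places EndOfTimeOffset a fixed distance beyond the first-person character's X location.
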(fn `UserConstructionScript`)