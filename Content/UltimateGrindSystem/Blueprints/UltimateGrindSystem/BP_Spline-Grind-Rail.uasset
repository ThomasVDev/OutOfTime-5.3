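; Grind rail actor for the Ultimate Grind System, supplying spline and grind settings to the character's grind component.
; The construction script builds query-only spline meshes between consecutive points.
; GetGrindSpline returns the rail's offset, speed, jump flag, effects, sounds, start distance and direction.
; Start distance comes from fixed-step sampling along the spline; two-way rails derive direction by comparing capsule yaw with spline yaw.
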(fn `CalculateDirection`
  (params (`Z_Value A` :type "Float (double-precision)") (`Z_Value B` :type "Float (double-precision)") (HitLocation :type "Vector Structure") (CharRef :type "Character Object Reference"))
  (returns (Direction :type "Float (double-precision)"))
  (locals (Z_ValueL :type "Float (double-precision)" :default 0.0))
  (bind _returnvalue (+ (`local.Z_ValueL`) (`local.Z_Value A`)))
  (bind _returnvalue_2 (+ (`local.Z_ValueL`) (`local.Z_Value B`)))
  (bind _returnvalue_3 (`KismetMathLibrary.NormalizeAxis` _returnvalue))
  (bind (_returnvalue_roll _returnvalue_pitch _returnvalue_yaw) (`KismetMathLibrary.BreakRotator` (`SceneComponent.K2_GetComponentRotation` (`Character.CapsuleComponent` (`local.CharRef`)))))
  (bind _returnvalue_4 (`KismetMathLibrary.NormalizeAxis` _returnvalue_2))
  (bind (_returnvalue_roll_2 _returnvalue_pitch_2 _returnvalue_yaw_2) (`KismetMathLibrary.BreakRotator` (`SceneComponent.K2_GetComponentRotation` (`Character.CapsuleComponent` (`local.CharRef`)))))
  (bind _returnvalue_5 (`KismetMathLibrary.NearlyEqual_FloatFloat` _returnvalue _returnvalue_3 0.1))
  (bind _returnvalue_6 (> (`local.Z_ValueL`) _returnvalue_3))
  (bind _returnvalue_7 (`KismetMathLibrary.NearlyEqual_FloatFloat` _returnvalue_2 _returnvalue_4 0.1))
  (bind _returnvalue_8 (> (`local.Z_ValueL`) _returnvalue_4))
  (bind (_returnvalue_roll_3 _returnvalue_pitch_3 _returnvalue_yaw_3) (`KismetMathLibrary.BreakRotator` (`SplineComponent.GetRotationAtDistanceAlongSpline` (`self.Spline`) (`SplineComponent.GetDistanceAlongSplineAtSplineInputKey` (`self.Spline`) (`SplineComponent.FindInputKeyClosestToWorldLocation` (`self.Spline`) (`SplineComponent.FindLocationClosestToWorldLocation` (`self.Spline`) (`local.HitLocation`) "World"))) "World")))
  (bind _returnvalue_9 (select `bool` _returnvalue_5 :`true` true))
  (bind _returnvalue_10 (select `bool` _returnvalue_7 :`true` true))
  (bind _returnvalue_11 (`KismetMathLibrary.InRange_FloatFloat` _returnvalue_yaw_2 (`KismetMathLibrary.SelectFloat` _returnvalue_4 (`local.Z_ValueL`) _returnvalue_8) (`KismetMathLibrary.SelectFloat` (`local.Z_ValueL`) _returnvalue_4 _returnvalue_8) _returnvalue_10 _returnvalue_10))
  (bind _returnvalue_12 (`KismetMathLibrary.InRange_FloatFloat` _returnvalue_yaw (`KismetMathLibrary.SelectFloat` _returnvalue_3 (`local.Z_ValueL`) _returnvalue_6) (`KismetMathLibrary.SelectFloat` (`local.Z_ValueL`) _returnvalue_3 _returnvalue_6) _returnvalue_9 _returnvalue_9))
  (set `local.Z_ValueL` _returnvalue_yaw_3)
  (return (`KismetMathLibrary.SelectFloat` 1.0 -1.0 (or (select `bool` _returnvalue_5 :`false` (not _returnvalue_12) :`true` _returnvalue_12) (select `bool` _returnvalue_7 :`false` (not _returnvalue_11) :`true` _returnvalue_11)))))

(fn `canGrind?`
  (returns (yes :type Boolean))
  (return true))

(fn `changeDATA`
  (params (NewSpeed :type "Float (double-precision)") (TypeDirecction :type "/Game/UltimateGrindSystem/Blueprints/UltimateGrindSystem/Components/BP_E_TypeDirecction Enum" :default "NewEnumerator0") (`IsJump?` :type Boolean) (FVX_FootLeft :type "ParticleSystem Object Reference") (FVX_FootRight :type "ParticleSystem Object Reference") (SVX_SoundLoop :type "SoundBase Object Reference"))
  (return))

(fn `getClosetDistanceAlongSpline`
  (params (location :type "Vector Structure"))
  (returns (splineDistance :type "Float (double-precision)"))
  (locals (DistanceSpline :type "Float (double-precision)" :default 0.0) (closetDistance :type "Float (double-precision)") (minDistance :type "Float (double-precision)" :default 119999985352704.0))
  (bind _distancespline (`local.DistanceSpline`))
  (bind _returnvalue (`KismetMathLibrary.Vector_Distance` location (`SplineComponent.GetLocationAtDistanceAlongSpline` (`self.Spline`) (`local.DistanceSpline`) "World")))
  (if (< _returnvalue (`local.minDistance`)) :!label _label
    (set `local.minDistance` _returnvalue)
    (set `local.closetDistance` (`local.DistanceSpline`)))
  (set `local.DistanceSpline` (+ _distancespline 10.0))
  (if (< _distancespline (`SplineComponent.GetSplineLength` (`self.Spline`)))
    (goto _label)
    (else
      (return (`local.closetDistance`)))))

(fn `getGrindSpline`
  (params (Location :type "Vector Structure") (HitLocation :type "Vector Structure") (Speed :type "Float (double-precision)") (charRef :type "Character Object Reference"))
  (returns (grindSpline :type "SplineComponent Object Reference") (starPoint :type "Float (double-precision)") (direction :type "Float (double-precision)") (grindOffset :type "Float (double-precision)") (SpeedSpline :type "Float (double-precision)") (`isJump?` :type Boolean) (FVX_FootLeft :type "ParticleSystem Object Reference") (FVX_FootRight :type "ParticleSystem Object Reference") (`SVX_Loop-SoundLoop` :type "SoundBase Object Reference") (`SVX_Start-Sound` :type "SoundBase Object Reference") (`SVX_End-Sound` :type "SoundBase Object Reference"))
  ;[0 0 0] This function is requested from the "Ultimate Grind System" component of the character and sends all the information of the Spline
  (bind _splinedistance (`self.getClosetDistanceAlongSpline` Location))
  (return (`self.Spline`) _splinedistance (select `/Game/UltimateGrindSystem/Blueprints/UltimateGrindSystem/Components/BP_E_TypeDirecction` (`self.TypeDirecction`) :`NewEnumerator0` 1.0 :`NewEnumerator1` (`self.CalculateDirection` 90.0 -90.0 (`local.HitLocation`) (`local.charRef`))) (`self.Grind Offset`) (`self.SpeedSpline`) (`self.Is Jump?`) (`self.FVX Foot Left`) (`self.FVX Foot Right`) (`self.SVX Sound Loop`) (`self.SVX Start- Sound`) (`self.SVX End- Sound`)))

(fn `UserConstructionScript`
  (bind _spline (`self.Spline`))
  ;[0 0 0] Spline Grind
  (for _index (range (+ (- (`SplineComponent.GetNumberOfSplinePoints` (`self.Spline`)) 2) 1))
    (bind _returnvalue (`AddComponent|NODE_AddSplineMeshComponent-0`))
    (`StaticMeshComponent.SetStaticMesh` _returnvalue (`self.StaticMesh`))
    (`SplineMeshComponent.SetForwardAxis` _returnvalue (`self.In Forward Axis`) true)
    (`SceneComponent.K2_AttachToComponent` _returnvalue (`self.Spline`) "None" "KeepRelative" "KeepRelative" "KeepRelative" true)
    (bind _returnvalue_2 (+ _index 1))
    (`SplineMeshComponent.SetStartAndEnd` _returnvalue (`SplineComponent.GetLocationAtSplinePoint` _spline _index "Local") (`SplineComponent.GetTangentAtSplinePoint` _spline _index "Local") (`SplineComponent.GetLocationAtSplinePoint` _spline _returnvalue_2 "Local") (`SplineComponent.GetTangentAtSplinePoint` _spline _returnvalue_2 "Local") true)
    (`PrimitiveComponent.SetCollisionEnabled` _returnvalue "QueryOnly")))