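; Collectible coin pickup for the Ultimate Grind System, awarded when a Character overlaps its sphere.
; Overlap adds one coin through the character's C_UltimateGrindSystem component, unless its coin system is disabled, and plays a sound.
; The item then destroys itself or, if IsRegenerate is set, hides while a one-second looping timer counts down to respawn.
; DoOnce gates prevent repeat triggers; grind functions are stubs marking it non-grindable.
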(event `self.ReceiveBeginPlay`
  ;[0 0 0] Begin Play
  ;[0 0 0] Setup regenerate
  (if (`self.isRegenerate?`)
    (set `self.itemActive?` true)
    (set `self.liveRenegerate` (`self.timeRegenerate`))))

(event `StopLiveItem`
  ;[0 0 0] Stop and Remove the Timer to optimize the coin system
  (`/Engine/EditorBlueprintResources/StandardMacros.DoOnce` false :!label _label
    (:`Completed`
      (`KismetSystemLibrary.Delay` 0.2)
      (`KismetSystemLibrary.K2_ClearAndInvalidateTimerHandle` (`self.TimerLiveItem`))
      (`self.ResetStop`))))

(event `ResetStop`
  ;[0 0 0] Stop and Remove the Timer to optimize the coin system
  (goto _label :!via `Reset`))

(event `RegenerationLiveItem`
  ;[0 0 0] Setup regenerate
  (`/Engine/EditorBlueprintResources/StandardMacros.DoOnce` false :!label _label_2
    (:`Completed`
      (set `self.liveRenegerate` (`self.timeRegenerate`))
      (bind _returnvalue (`KismetSystemLibrary.K2_SetTimer` null "RegenerateItem" 1.0 true))
      (set `self.TimerLiveItem` _returnvalue))))

(event `ResetRegeneration`
  ;[0 0 0] Setup regenerate
  (goto _label_2 :!via `Reset`))

(event `self.Sphere.OnComponentBeginOverlap`
  (params (OverlappedComponent :type "PrimitiveComponent Object Reference") (OtherActor :type "Actor Object Reference") (OtherComp :type "PrimitiveComponent Object Reference") (OtherBodyIndex :type Integer) (bFromSweep :type Boolean) (SweepResult :type "HitResult Structure (by ref)"))
  (bind _ascharacter (cast `Character` OtherActor))
  (bind _returnvalue (`self.GetComponentByClass` _ascharacter "/Game/UltimateGrindSystem/Blueprints/UltimateGrindSystem/Components/C_UltimateGrindSystem.C_UltimateGrindSystem_C"))
  (if (not (`/Game/UltimateGrindSystem/Blueprints/UltimateGrindSystem/Components/C_UltimateGrindSystem.DisableCoinSystem?` _returnvalue))
    ;[0 0 0] Item collection system when colliding with a character
    (`/Engine/EditorBlueprintResources/StandardMacros.DoOnce` false :!label _label_3
      (:`Completed`
        ;;[0 0 0 1 10] Send 1 or more items to the character's UltimateGrindSystem component
        (message `/Game/UltimateGrindSystem/Blueprints/UltimateGrindSystem/Components/BPI_Grind.collectCoin` _returnvalue 1)
        (`GameplayStatics.PlaySound2D` "/Game/UltimateGrindSystem/Environment/SVX/Cue_SoundCoin.Cue_SoundCoin" 1.0 1.0 0.0 null null)
        ;;[0 0 0 1 12] Restarts the regeneration if it is activated; if it is false the whole actor is destroyed
        (if (`self.isRegenerate?`)
          (`SceneComponent.SetHiddenInGame` (`self.CoinMesh`) true false)
          (set `self.itemActive?` false)
          (`self.RegenerationLiveItem`)
          (else
            (`self.K2_DestroyActor`)))))))

(event `ResetItem`
  (`self.ResetRegeneration`)
  (goto _label_3 :!via `Reset`))

(fn `canGrind?`
  (returns (yes :type Boolean))
  (return false))

(fn `getGrindSpline`
  (params (Location :type "Vector Structure") (HitLocation :type "Vector Structure") (Speed :type "Float (double-precision)") (charRef :type "Character Object Reference"))
  (returns (grindSpline :type "SplineComponent Object Reference") (starPoint :type "Float (double-precision)") (direction :type "Float (double-precision)") (grindOffset :type "Float (double-precision)") (SpeedSpline :type "Float (double-precision)") (`isJump?` :type Boolean) (FVX_FootLeft :type "ParticleSystem Object Reference") (FVX_FootRight :type "ParticleSystem Object Reference") (`SVX_Loop-SoundLoop` :type "SoundBase Object Reference") (`SVX_Start-Sound` :type "SoundBase Object Reference") (`SVX_End-Sound` :type "SoundBase Object Reference"))
  (return null 0.0 0.0 0.0 0.0 false null null null null null))

(fn `RegenerateItem`
  (if (not (`self.itemActive?`))
    (set `self.liveRenegerate` (`KismetMathLibrary.Clamp` (- (`self.liveRenegerate`) 1) 0 (`self.timeRegenerate`)))
    (if (<= (`self.liveRenegerate`) 0)
      (set `self.liveRenegerate` (`self.timeRegenerate`))
      (`self.ResetItem`)
      (`SceneComponent.SetHiddenInGame` (`self.CoinMesh`) false false)
      (set `self.itemActive?` true)
      (`self.StopLiveItem`))))

(fn `UserConstructionScript`
  (`StaticMeshComponent.SetStaticMesh` (`self.CoinMesh`) (`self.StaticMesh`)))