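; BP_Spline-ITEM lays out a row of items, such as coins, along a spline in the Ultimate Grind System.
; The construction script builds evenly spaced preview meshes with configurable count and scale, optionally oriented to the spline.
; On BeginPlay it spawns a BP_Item at each preview transform, passing mesh and regeneration settings, then destroys the preview.
; Its grind functions are stubs, though CanGrind returns true.
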(event `self.ReceiveBeginPlay`
  ;[0 0 0] Begin play
  ;;[0 0 0] Creation of item according to the configuration of the construction
  (for (_array_element _array_index) (`self.MeshComponet`)
    (`|SpawnActorFromClass` "/Game/UltimateGrindSystem/Blueprints/UltimateGrindSystem/BP_Item.BP_Item_C" (`SceneComponent.K2_GetComponentToWorld` _array_element) "AdjustIfPossibleButAlwaysSpawn" "OverrideRootScale" null (`self.Is Regenerate?`) (`self.Time Regenerate`) (`self.StaticMesh`) null)
    ;;[0 0 0] Destruction of the reference component of the construction
    (`ActorComponent.K2_DestroyComponent` (`|GetArrayItem` (`self.MeshComponet`) _array_index))))

(fn `canGrind?`
  (returns (yes :type Boolean))
  (return true))

(fn `changeDATA`
  (params (NewSpeed :type "Float (double-precision)") (TypeDirecction :type "/Game/UltimateGrindSystem/Blueprints/UltimateGrindSystem/Components/BP_E_TypeDirecction Enum" :default "NewEnumerator0") (`IsJump?` :type Boolean) (FVX_FootLeft :type "ParticleSystem Object Reference") (FVX_FootRight :type "ParticleSystem Object Reference") (SVX_SoundLoop :type "SoundBase Object Reference"))
  (return))

(fn `getGrindSpline`
  (params (Location :type "Vector Structure") (HitLocation :type "Vector Structure") (Speed :type "Float (double-precision)") (charRef :type "Character Object Reference"))
  (returns (grindSpline :type "SplineComponent Object Reference") (starPoint :type "Float (double-precision)") (direction :type "Float (double-precision)") (grindOffset :type "Float (double-precision)") (SpeedSpline :type "Float (double-precision)") (`isJump?` :type Boolean) (FVX_FootLeft :type "ParticleSystem Object Reference") (FVX_FootRight :type "ParticleSystem Object Reference") (`SVX_Loop-SoundLoop` :type "SoundBase Object Reference") (`SVX_Start-Sound` :type "SoundBase Object Reference") (`SVX_End-Sound` :type "SoundBase Object Reference"))
  (return null 0.0 1.0 0.0 0.0 false null null null null null))

(fn `UserConstructionScript`
  (bind _number_of_coins (`self.Number of Coins`))
  (bind _scalecoins (`self.ScaleCoins`))
  (bind _returnvalue (- _number_of_coins 1))
  ;[0 0 0] Spline - ItemSystem
  (if (> _number_of_coins 0)
    (for _index (range (+ _returnvalue 1))
      (bind _returnvalue_2 (* _index (/ (`SplineComponent.GetSplineLength` (`self.Spline1`)) (`KismetMathLibrary.Conv_IntToDouble` _returnvalue))))
      (bind _returnvalue_3 (`KismetMathLibrary.MakeTransform` (`KismetMathLibrary.InverseTransformLocation` (`self.GetTransform`) (`SplineComponent.GetLocationAtDistanceAlongSpline` (`self.Spline1`) _returnvalue_2 "World")) (struct) (`KismetMathLibrary.MakeVector` _scalecoins _scalecoins _scalecoins)))
      ;;[0 0 0] Referential mesh configuration
      (bind _returnvalue_4 (`AddComponent|NODE_AddStaticMeshComponent-0` :`RelativeTransform` _returnvalue_3))
      (`StaticMeshComponent.SetStaticMesh` _returnvalue_4 (`self.StaticMesh`))
      ;;[0 0 0] The location of each item and the mesh is saved in an array so that when starting the game the items can be created correctly
      (`KismetArrayLibrary.Array_Add` (`self.TransformationCoin`) _returnvalue_3)
      (`KismetArrayLibrary.Array_Add` (`self.MeshComponet`) _returnvalue_4)
      (if (`self.Orient to spline`)
        (`SceneComponent.K2_SetWorldRotation` _returnvalue_4 (`SplineComponent.GetRotationAtDistanceAlongSpline` (`self.Spline1`) _returnvalue_2 "World") false false)))))