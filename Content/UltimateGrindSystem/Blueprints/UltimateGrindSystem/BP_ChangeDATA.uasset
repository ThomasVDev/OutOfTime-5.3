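; BP_ChangeDATA is a trigger actor that changes a character's active grind settings in the Ultimate Grind System.
; When a Character overlaps DetectCharacter, it passes its speed, direction type, jump flag, foot effects and looping sound to that character's C_UltimateGrindSystem component through ChangeDATAMessage.
; Its CanGrind and GetGrindSpline functions return false and zero defaults, so it offers no grindable spline itself.
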(event `self.DetectCharacter.OnComponentBeginOverlap`
  (params (OverlappedComponent :type "PrimitiveComponent Object Reference") (OtherActor :type "Actor Object Reference") (OtherComp :type "PrimitiveComponent Object Reference") (OtherBodyIndex :type Integer) (bFromSweep :type Boolean) (SweepResult :type "HitResult Structure (by ref)"))
  ;[0 0 0] Send new custom spline information to the character's "Ultimate Grind System" component
  (bind _ascharacter (cast `Character` OtherActor))
  (message `/Game/UltimateGrindSystem/Blueprints/UltimateGrindSystem/Components/BPI_Grind.changeDATA` (`self.GetComponentByClass` _ascharacter "/Game/UltimateGrindSystem/Blueprints/UltimateGrindSystem/Components/C_UltimateGrindSystem.C_UltimateGrindSystem_C") (`self.SpeedSpline`) (`self.Type Direcction`) (`self.Is Jump?`) (`self.FVX Foot Left`) (`self.FVX Foot Right`) (`self.SVX Sound Loop`)))

(fn `canGrind?`
  (returns (yes :type Boolean))
  (return false))

(fn `getGrindSpline`
  (params (Location :type "Vector Structure") (HitLocation :type "Vector Structure") (Speed :type "Float (double-precision)") (charRef :type "Character Object Reference"))
  (returns (grindSpline :type "SplineComponent Object Reference") (starPoint :type "Float (double-precision)") (direction :type "Float (double-precision)") (grindOffset :type "Float (double-precision)") (SpeedSpline :type "Float (double-precision)") (`isJump?` :type Boolean) (FVX_FootLeft :type "ParticleSystem Object Reference") (FVX_FootRight :type "ParticleSystem Object Reference") (`SVX_Loop-SoundLoop` :type "SoundBase Object Reference") (`SVX_Start-Sound` :type "SoundBase Object Reference") (`SVX_End-Sound` :type "SoundBase Object Reference"))
  (return null 0.0 0.0 0.0 0.0 false null null null null null))

(fn `UserConstructionScript`)