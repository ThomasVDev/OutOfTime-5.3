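; Turret actor that, while its sensor is toggled on by Spotted/NotSpotted events, tracks and shoots at first-person player characters.
; Each tick it sphere-overlaps for the nearest character with line of sight, then rotates toward it at constant speed with clamped yaw.
; When the cooldown has elapsed and a dot-product check confirms aim, it spawns a timed burst of bullets from the FirePlace socket using a DoN/Delay loop.
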(event `self.ReceiveTick`
  (params (DeltaSeconds :type "Float (single-precision)"))
  (if (`self.NeedsSensor`)
    (`self.FindBestTarget`)
    (`self.Target`
      (:`then`
        (`self.Update Turret Rotation` DeltaSeconds)
        (`self.UpdateFire`))
      (:`else`))))

(event `Fire`
  (set `self.TimeOfLastFire` (`KismetSystemLibrary.GetGameTimeInSeconds`))
  (`|ExecutionSequence`
    (:`then_0`
      (goto _label :!via `Reset`))
    (:`then_1`
      (`/Engine/EditorBlueprintResources/StandardMacros.Do N` (`self.ShotsPerRound`) :!label _label
        (:`Exit`
          (`|SpawnActorFromClass` (`self.Bullet`) (`SceneComponent.GetSocketTransform` (`self.Turret`) "FirePlace" "RTS_World") "Undefined" "SelectDefaultAtRuntime" null null)
          (`KismetSystemLibrary.Delay` 0.3)
          (goto _label))))))

(event `/Game/Blueprints/BlueprintInterfaces/BPI_TurretSensing.NotSpotted`
  (set `self.NeedsSensor` false))

(event `/Game/Blueprints/BlueprintInterfaces/BPI_TurretSensing.Spotted`
  (set `self.NeedsSensor` true))

(fn `FindBestTarget`
  (locals (`BestDistance (local)` :type "Float (double-precision)") (`CurrentDistance (local)` :type "Float (double-precision)") (`BestTarget (local)` :type "Actor Object Reference") (`CurrentTarget (local)` :type "Actor Object Reference"))
  (bind _besttarget (`self.BestTarget`))
  (set `local.BestDistance (local)` (+ (`self.SensingRange`) 1.0))
  (bind _outactors (`KismetSystemLibrary.SphereOverlapActors` (`self.K2_GetActorLocation`) (`self.SensingRange`) (`|MakeArray` "ObjectTypeQuery3" :!type "EObjectTypeQuery Enum") "/Game/Blueprints/BP_FirstPersonCharacter.BP_FirstPersonCharacter_C"))
  (for _array_element _outactors
    (bind _output_get (set `local.CurrentTarget (local)` _array_element))
    (bind _output_get_2 (set `local.CurrentDistance (local)` (`self.GetDistanceTo` _output_get self)))
    (if (or (< _output_get_2 (`local.BestDistance (local)`)) (not (`KismetSystemLibrary.IsValid` _besttarget)))
      (bind _return (`/Game/FunctionLibraries/LineOfSight.HasLineOfSight` (`SceneComponent.K2_GetComponentLocation` (`self.Turret`)) (`self.K2_GetActorLocation` (`local.CurrentTarget (local)`)) (`|MakeArray` self (`local.CurrentTarget (local)`) :!type "Actor Object Reference")))
      (if _return
        (set `self.BestTarget` (`local.CurrentTarget (local)`))
        (set `local.BestDistance (local)` (`local.CurrentDistance (local)`)))))
  (set `self.Target` _besttarget))

(fn `Update Turret Rotation`
  (params (DeltaSeconds :type "Float (double-precision)"))
  (locals (NewRotation :type "Rotator Structure" :default (struct)))
  (bind _turret (`self.Turret`))
  (bind _output_get (set `local.NewRotation` (`KismetMathLibrary.RInterpTo_Constant` (`SceneComponent.K2_GetComponentRotation` _turret) (`KismetMathLibrary.FindLookAtRotation` (`SceneComponent.GetSocketLocation` _turret "FirePlace") (`self.K2_GetActorLocation` (`self.Target`))) (`local.DeltaSeconds`) (`self.TurretRotationSpeed`))))
  (`SceneComponent.K2_SetWorldRotation` (`self.Turret`) (`KismetMathLibrary.MakeRotator` (.roll _output_get) (.pitch _output_get) (`KismetMathLibrary.ClampAngle` (.yaw _output_get) (`self.Min Angle Degrees`) (`self.Max Angle Degrees`))) true false))

(fn `UpdateFire`
  (if (> (- (`KismetSystemLibrary.GetGameTimeInSeconds`) (`self.TimeOfLastFire`)) (`self.RateOfFire`))
    (if (> (`KismetMathLibrary.Dot_VectorVector` (`KismetMathLibrary.GetDirectionUnitVector` (`SceneComponent.K2_GetComponentLocation` (`self.Turret`)) (`self.K2_GetActorLocation` (`self.Target`))) (`SceneComponent.GetForwardVector` (`self.Turret`))) 0.98)
      (`self.Fire`))))

(fn `UserConstructionScript`)