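; BP_SpiderwebProjectile is a turret obstacle projectile that can kill the first-person player on contact.
; When its Sphere overlaps the player's capsule, an active TimeShield triggers time stop and the shield cooldown, then destroys the projectile; otherwise the player dies.
; Overlapping any other actor destroys the projectile after a short delay.
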(event `self.Sphere.OnComponentBeginOverlap`
  (params (OverlappedComponent :type "PrimitiveComponent Object Reference") (OtherActor :type "Actor Object Reference") (OtherComp :type "PrimitiveComponent Object Reference") (OtherBodyIndex :type Integer) (bFromSweep :type Boolean) (SweepResult :type "HitResult Structure (by ref)"))
  (bind _asbp_first_person_character (cast `/Game/Blueprints/BP_FirstPersonCharacter` OtherActor :!pure true))
  (if (== (`GameplayStatics.GetObjectClass` OtherActor) "/Game/Blueprints/BP_FirstPersonCharacter.BP_FirstPersonCharacter_C")
    (if (`PrimitiveComponent.IsOverlappingComponent` (`Character.CapsuleComponent` _asbp_first_person_character) (`self.Sphere`))
      (if (`/Game/Blueprints/BP_FirstPersonCharacter.TimeShield` _asbp_first_person_character)
        (`/Game/Blueprints/BP_FirstPersonCharacter.Start Time Stop` _asbp_first_person_character)
        (`/Game/Blueprints/BP_FirstPersonCharacter.CooldownTimeShield` _asbp_first_person_character)
        (`self.K2_DestroyActor`)
        (else
          (`/Game/Blueprints/BP_FirstPersonCharacter.Die` _asbp_first_person_character))))
    (else
      (`KismetSystemLibrary.Delay` 3.0)
      (`self.K2_DestroyActor`))))

(fn `UserConstructionScript`)