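; BP_Sensor is a detection sphere that tells turrets when the first-person player is spotted or lost.
; Sphere overlap begin and end message actors implementing BPI_TurretSensing and toggle InSight.
; On entry, a Timeline's updates sweep the sphere to the player's location, pausing movement while the player's StopTime is set.
; On exit, the actor sweeps back to its BeginPlay location, with no call to stop the Timeline.
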(event `FollowPlayer`
  (bind _asbp_first_person_character (cast `/Game/Blueprints/BP_FirstPersonCharacter` (`GameplayStatics.GetPlayerPawn` 0) :!pure true))
  (if (not (`/Game/Blueprints/BP_FirstPersonCharacter.StopTime?` _asbp_first_person_character))
    (`SceneComponent.K2_SetWorldLocation` (`self.Sphere`) (`self.K2_GetActorLocation` _asbp_first_person_character) true false)))

(event `self.ReceiveBeginPlay`
  (set `self.Alocation` (`self.K2_GetActorLocation`)))

(event `self.Sphere.OnComponentBeginOverlap`
  (params (OverlappedComponent :type "PrimitiveComponent Object Reference") (OtherActor :type "Actor Object Reference") (OtherComp :type "PrimitiveComponent Object Reference") (OtherBodyIndex :type Integer) (bFromSweep :type Boolean) (SweepResult :type "HitResult Structure (by ref)"))
  (if (== (`GameplayStatics.GetObjectClass` (cast `/Game/Blueprints/BP_FirstPersonCharacter` OtherActor :!pure true)) "/Game/Blueprints/BP_FirstPersonCharacter.BP_FirstPersonCharacter_C")
    (`GameplayStatics.GetAllActorsWithInterface` "/Game/Blueprints/BlueprintInterfaces/BPI_TurretSensing.BPI_TurretSensing_C")
    (message `/Game/Blueprints/BlueprintInterfaces/BPI_TurretSensing.Spotted` (`self.Turrets`))
    (set `self.InSight` true)
    (`Timeline|Timeline`
      (:`Update`
        (`self.FollowPlayer`)))))

(event `self.Sphere.OnComponentEndOverlap`
  (params (OverlappedComponent :type "PrimitiveComponent Object Reference") (OtherActor :type "Actor Object Reference") (OtherComp :type "PrimitiveComponent Object Reference") (OtherBodyIndex :type Integer))
  (if (== (`GameplayStatics.GetObjectClass` (cast `/Game/Blueprints/BP_FirstPersonCharacter` OtherActor :!pure true)) "/Game/Blueprints/BP_FirstPersonCharacter.BP_FirstPersonCharacter_C")
    (`GameplayStatics.GetAllActorsWithInterface` "/Game/Blueprints/BlueprintInterfaces/BPI_TurretSensing.BPI_TurretSensing_C")
    (message `/Game/Blueprints/BlueprintInterfaces/BPI_TurretSensing.NotSpotted` (`self.Turrets`))
    (set `self.InSight` false)
    (`self.K2_SetActorLocation` (`self.Alocation`) true)))

(fn `UserConstructionScript`)