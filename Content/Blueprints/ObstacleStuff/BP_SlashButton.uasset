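; BP_SlashButton is a button that the player triggers with an attack, activating linked obstacles or other objects.
; On BeginPlay its cube gets a green lamp material, and a red lamp material is created for the activated state.
; When an overlap begins and the cube touches the first-person character's AttackRange, it sends ActivateMessage to every entry in ActivatableObjects and switches to red.
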(event `self.ReceiveBeginPlay`
  (bind _returnvalue (`KismetMaterialLibrary.CreateDynamicMaterialInstance` "/Game/PrototypeMaterials/M_SuperGrid_GreenLamp.M_SuperGrid_GreenLamp"))
  (`PrimitiveComponent.SetMaterial` (`self.Cube`) 0 _returnvalue)
  (bind _returnvalue_2 (`KismetMaterialLibrary.CreateDynamicMaterialInstance` "/Game/PrototypeMaterials/M_SuperGrid_RedLamp.M_SuperGrid_RedLamp"))
  (set `self.ActivatedMat` _returnvalue_2))

(event `self.Cube.OnComponentBeginOverlap`
  (params (OverlappedComponent :type "PrimitiveComponent Object Reference") (OtherActor :type "Actor Object Reference") (OtherComp :type "PrimitiveComponent Object Reference") (OtherBodyIndex :type Integer) (bFromSweep :type Boolean) (SweepResult :type "HitResult Structure (by ref)"))
  (if (`PrimitiveComponent.IsOverlappingComponent` (`self.Cube`) (`/Game/Blueprints/BP_FirstPersonCharacter.AttackRange` (`self.GetPlayer`)))
    (for _array_element (`self.ActivatableObjects`)
      (message `/Game/Blueprints/BlueprintInterfaces/BPI_Activatable.Activate` _array_element))
    (`PrimitiveComponent.SetMaterial` (`self.Cube`) 0 (`self.ActivatedMat`))))

(fn `GetPlayer`
  (returns (`AsBP First Person Character` :type "/Game/Blueprints/BP_FirstPersonCharacter Object Reference"))
  (return (cast `/Game/Blueprints/BP_FirstPersonCharacter` (`GameplayStatics.GetPlayerCharacter` 0) :!pure true)))

(fn `UserConstructionScript`)