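; BP_AirVent is an air vent obstacle that pushes the first-person character along its Arrow's forward direction.
; Entering the Box while StopTime is off re-enables jumping and starts a self-calling event loop.
; The loop stops any slide and adds launch velocity every 0.2 seconds until the character leaves the Box.
; StopTime is checked only on entry, not during the loop.
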(event `self.Box.OnComponentBeginOverlap`
  (params (OverlappedComponent :type "PrimitiveComponent Object Reference") (OtherActor :type "Actor Object Reference") (OtherComp :type "PrimitiveComponent Object Reference") (OtherBodyIndex :type Integer) (bFromSweep :type Boolean) (SweepResult :type "HitResult Structure (by ref)"))
  (bind _asbp_first_person_character (cast `/Game/Blueprints/BP_FirstPersonCharacter` OtherActor))
  (bind _output_get (set `self.As BP First Person Character` _asbp_first_person_character))
  (if (`/Game/Blueprints/BP_FirstPersonCharacter.StopTime?` _asbp_first_person_character)
    _
    (elif (`PrimitiveComponent.IsOverlappingComponent` (`self.Box`) (`Character.CapsuleComponent` _output_get))
      (set `self.PlayerStillThere` true)
      (`self.Is overlapping`)
      (set `/Game/Blueprints/BP_FirstPersonCharacter.JumpAllowed` true _asbp_first_person_character))))

(event `Is overlapping`
  (`/Game/Blueprints/BP_FirstPersonCharacter.StopSlide` (`self.As BP First Person Character`))
  (if (`self.PlayerStillThere`)
    (`Character.LaunchCharacter` (`self.As BP First Person Character`) (* (`SceneComponent.GetForwardVector` (`self.Arrow`)) (`self.LaunchVel`)) false false)
    (`KismetSystemLibrary.Delay` 0.2)
    (`self.Is overlapping`)))

(event `self.Box.OnComponentEndOverlap`
  (params (OverlappedComponent :type "PrimitiveComponent Object Reference") (OtherActor :type "Actor Object Reference") (OtherComp :type "PrimitiveComponent Object Reference") (OtherBodyIndex :type Integer))
  (cast `/Game/Blueprints/BP_FirstPersonCharacter` OtherActor)
  (set `self.PlayerStillThere` false))

(fn `UserConstructionScript`)