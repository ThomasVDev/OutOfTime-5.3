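; BP_FloorButton is a pressure-plate floor button that triggers linked objects when a player or physics-simulating item stands on it.
; Box overlap begin plays a timeline that lowers Cylinder1 and sends ActivateMessage to every ActivateObjects entry implementing BPI_Activatable.
; Overlap end reverses the timeline and sends DeactivateMessage, but only once no simulating components or overlapping actors remain in the Box.
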(event `DownAnim`
  (bind (_direction _zoffset) (`Timeline|ButtonDown` :!label _label)
    (:`Update`
      (`SceneComponent.K2_SetRelativeLocation` (`self.Cylinder1`) (`KismetMathLibrary.MakeVector` 0.0 0.0 _zoffset) false false))))

(event `UpAnim`
  (goto _label :!via `Reverse`))

(event `self.Box.OnComponentBeginOverlap`
  (params (OverlappedComponent :type "PrimitiveComponent Object Reference") (OtherActor :type "Actor Object Reference") (OtherComp :type "PrimitiveComponent Object Reference") (OtherBodyIndex :type Integer) (bFromSweep :type Boolean) (SweepResult :type "HitResult Structure (by ref)"))
  (bind _returnvalue (`self.IsPlayerOrPhysicsItem` OtherActor OtherComp))
  (if _returnvalue
    (`self.DownAnim`)
    (for _array_element (`self.ActivateObjects`)
      (if (`KismetSystemLibrary.DoesImplementInterface` _array_element "/Game/Blueprints/BlueprintInterfaces/BPI_Activatable.BPI_Activatable_C")
        (message `/Game/Blueprints/BlueprintInterfaces/BPI_Activatable.Activate` _array_element)))))

(event `self.Box.OnComponentEndOverlap`
  (params (OverlappedComponent :type "PrimitiveComponent Object Reference") (OtherActor :type "Actor Object Reference") (OtherComp :type "PrimitiveComponent Object Reference") (OtherBodyIndex :type Integer))
  (bind _returnvalue (`self.IsPlayerOrPhysicsItem` OtherActor OtherComp))
  (if (and _returnvalue (`self.AreThereNotAnyObjectsOntopOfButton`))
    (`self.UpAnim`)
    (for _array_element (`self.ActivateObjects`)
      (if (`KismetSystemLibrary.DoesImplementInterface` _array_element "/Game/Blueprints/BlueprintInterfaces/BPI_Activatable.BPI_Activatable_C")
        (message `/Game/Blueprints/BlueprintInterfaces/BPI_Activatable.Deactivate` _array_element)))))

(fn `AreThereNotAnyObjectsOntopOfButton`
  (returns (Return :type Boolean))
  (locals (`IsObjectOnButton?` :type Boolean))
  (for _array_element (`PrimitiveComponent.GetOverlappingComponents` (`self.Box`))
    (if (`SceneComponent.IsSimulatingPhysics` _array_element "None")
      (set `local.IsObjectOnButton?` true)))
  (return (and (not (`local.IsObjectOnButton?`)) (== (`KismetArrayLibrary.Array_Length` (`PrimitiveComponent.GetOverlappingActors` (`self.Box`) null)) 0))))

(fn `IsPlayerOrPhysicsItem`
  (params (`Other Actor` :type "Object Object Reference") (`Other Component` :type "SceneComponent Object Reference"))
  (returns (ReturnValue :type Boolean))
  (return (or (== (`GameplayStatics.GetObjectClass` `Other Actor`) null) (`SceneComponent.IsSimulatingPhysics` `Other Component` "None"))))

(fn `UserConstructionScript`)