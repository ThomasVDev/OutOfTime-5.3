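; BP_WallShocker is a shock hazard that repeatedly spawns BP_WallShock waves at its static mesh's transform.
; After a start delay it enables its linked receiver, if valid, and starts spawning unless it needs to be turned on.
; SpawnWaves loops by calling itself after each delay.
; Separate events disable the receiver and, on death, start the waves of other linked shockers in OtherSensorsTurnOn.
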(event `self.ReceiveBeginPlay`
  (bind _revciever (`self.Revciever`))
  (`KismetSystemLibrary.Delay` (`self.StartDelay`))
  (`/Engine/EditorBlueprintResources/StandardMacros.IsValid` _revciever
    (:`Is Valid`
      (`/Game/Blueprints/Enemies/Shocker/BP_WallShockReciever.Enable` _revciever))
    (:`Is Not Valid`
      _))
  (if (not (`self.Needs to be turned on`))
    (`self.SpawnWaves`)))

(event `SpawnWaves`
  (`KismetSystemLibrary.Delay` (`self.Delay Between `))
  (`|SpawnActorFromClass` "/Game/Blueprints/Enemies/Shocker/BP_WallShock.BP_WallShock_C" (`SceneComponent.K2_GetComponentToWorld` (`self.StaticMesh`)) "AlwaysSpawn" "MultiplyWithRoot" null null)
  (`self.SpawnWaves`))

(event `DisableReciever`
  (`/Game/Blueprints/Enemies/Shocker/BP_WallShockReciever.Disable` (`self.Revciever`)))

(event `OnDeathTurnOn`
  (bind _othersensorsturnon (`self.OtherSensorsTurnOn`))
  (if (`KismetArrayLibrary.Array_IsValidIndex` _othersensorsturnon)
    (for _array_element _othersensorsturnon
      (`self.SpawnWaves` _array_element))))

(fn `UserConstructionScript`)