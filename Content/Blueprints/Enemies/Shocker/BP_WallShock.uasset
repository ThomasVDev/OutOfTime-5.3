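; BP_WallShock is a short-lived Shocker enemy hazard that kills the first-person player on contact.
; It destroys itself once its LifeTime delay runs out after BeginPlay.
; Its Sphere overlap compares exact classes, calling Die on BP_FirstPersonCharacter or destroying the shock when it touches a BP_WallShockReciever.
; Killing the player does not destroy the shock, and other overlapping actors are ignored.
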(event `self.ReceiveBeginPlay`
  (`KismetSystemLibrary.Delay` (`self.LifeTime`))
  (`self.K2_DestroyActor` self))

(event `self.Sphere.OnComponentBeginOverlap`
  (params (OverlappedComponent :type "PrimitiveComponent Object Reference") (OtherActor :type "Actor Object Reference") (OtherComp :type "PrimitiveComponent Object Reference") (OtherBodyIndex :type Integer) (bFromSweep :type Boolean) (SweepResult :type "HitResult Structure (by ref)"))
  (bind _returnvalue (`GameplayStatics.GetObjectClass` OtherActor))
  (if (== _returnvalue "/Game/Blueprints/BP_FirstPersonCharacter.BP_FirstPersonCharacter_C")
    (`/Game/Blueprints/BP_FirstPersonCharacter.Die` (cast `/Game/Blueprints/BP_FirstPersonCharacter` OtherActor :!pure true))
    (elif (== _returnvalue "/Game/Blueprints/Enemies/Shocker/BP_WallShockReciever.BP_WallShockReciever_C")
      (`self.K2_DestroyActor`))))

(fn `UserConstructionScript`)