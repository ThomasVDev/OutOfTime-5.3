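; EnemySpawner is a placed actor that spawns the enemy type chosen by its WhatEnemy enum, such as DragonFly or SimpleShooting, at its Box.
; One tick after BeginPlay it maps the enum to a class and spawns it.
; The enemy is linked to NearestDoor, added to that door's Enemies list and given any roam points.
; MaybeSpawnNewOne repeats this only when the previous enemy is no longer valid.
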(event `self.ReceiveBeginPlay`
  (bind _map (`|MakeMap` "NewEnumerator0" null "NewEnumerator1" "/Game/Blueprints/Enemies/DragonFly/BP_DragonFlyTest.BP_DragonFlyTest_C" "NewEnumerator2" "/Game/Blueprints/Enemies/BP_SimpleShooter.BP_SimpleShooter_C" :!type "/Game/Blueprints/Enemies/E_EnemySpawner Enum" :!valuetype "/Game/Blueprints/Enemies/BP_Enemy Class Reference"))
  (bind _whatenemy (`self.WhatEnemy`))
  (bind _givenroampoints (`self.GivenRoamPoints`))
  (bind (_value _returnvalue) (`BlueprintMapLibrary.Map_Find` _map _whatenemy))
  (bind (_returnvalue_location _returnvalue_rotation) (`KismetMathLibrary.BreakTransform` (`SceneComponent.K2_GetComponentToWorld` (`self.Box`))))
  (`KismetSystemLibrary.DelayUntilNextTick`)
  (set `self.EnumToClass` _map)
  (switch `/Game/Blueprints/Enemies/E_EnemySpawner` _whatenemy
    (:`NewEnumerator0`
      _)
    (:`NewEnumerator1`
      _)
    (:`NewEnumerator2`
      _))
  (if _returnvalue
    (bind _returnvalue_2 (`|SpawnActorFromClass` _value (`KismetMathLibrary.MakeTransform` _returnvalue_location _returnvalue_rotation) "Undefined" "MultiplyWithRoot" null null))
    (bind _output_get (set `self.SpawnedEnemy` _returnvalue_2))
    (bind _output_get_2 (set `/Game/Blueprints/Enemies/BP_Enemy.Door` (`self.NearestDoor`) _output_get))
    (`KismetArrayLibrary.Array_AddUnique` (`/Game/Blueprints/ObstacleStuff/BP_Door.Enemies` _output_get_2) _output_get)
    (if (`KismetArrayLibrary.Array_IsValidIndex` _givenroampoints)
      (set `/Game/Blueprints/Enemies/BP_Enemy.RoamPoints` _givenroampoints _output_get))))

(event `MaybeSpawnNewOne`
  (bind _givenroampoints (`self.GivenRoamPoints`))
  (bind (_returnvalue_location _returnvalue_rotation) (`KismetMathLibrary.BreakTransform` (`SceneComponent.K2_GetComponentToWorld` (`self.Box`))))
  (bind (_value _returnvalue) (`BlueprintMapLibrary.Map_Find` (`self.EnumToClass`) (`self.WhatEnemy`)))
  (`/Engine/EditorBlueprintResources/StandardMacros.IsValid` (`self.SpawnedEnemy`)
    (:`Is Not Valid`
      (if _returnvalue
        (bind _returnvalue_2 (`|SpawnActorFromClass` _value (`KismetMathLibrary.MakeTransform` _returnvalue_location _returnvalue_rotation) "Undefined" "MultiplyWithRoot" null null))
        (bind _output_get (set `self.SpawnedEnemy` _returnvalue_2))
        (bind _output_get_2 (set `/Game/Blueprints/Enemies/BP_Enemy.Door` (`self.NearestDoor`) _output_get))
        (`KismetArrayLibrary.Array_AddUnique` (`/Game/Blueprints/ObstacleStuff/BP_Door.Enemies` _output_get_2) _output_get)
        (if (`KismetArrayLibrary.Array_IsValidIndex` _givenroampoints)
          (set `/Game/Blueprints/Enemies/BP_Enemy.RoamPoints` _givenroampoints _output_get))))))

(fn `UserConstructionScript`)