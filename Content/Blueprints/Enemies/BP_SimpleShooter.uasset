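; BP_SimpleShooter is an enemy that smoothly rotates its capsule to face the player and fires spiderweb projectiles from its Cube.
; The Box trigger toggles CanShoot as the first-person character enters or leaves, gating a self-recalling, delay-based StartShooting loop.
; Alert extends the parent by calling StartShooting and destroying the Box.
; A BP_DragonFlyTest whose Collision overlaps the Weakpoint triggers KillEnemy two ticks later.
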(event `StartShooting`
  (bind (_returnvalue_location _returnvalue_rotation) (`KismetMathLibrary.BreakTransform` (`SceneComponent.K2_GetComponentToWorld` (`self.Cube`))))
  (if (`self.canShoot`)
    (`|SpawnActorFromClass` "/Game/Blueprints/ObstacleStuff/Turrets/BP_SpiderwebProjectile.BP_SpiderwebProjectile_C" (`KismetMathLibrary.MakeTransform` _returnvalue_location _returnvalue_rotation (2.0 1.0 1.0)) "Undefined" "MultiplyWithRoot" null null)
    (`KismetSystemLibrary.Delay` (`self.TimeInBetweenShots`))
    (`self.StartShooting`)))

(event `self.ReceiveTick`
  (params (DeltaSeconds :type "Float (single-precision)"))
  (bind _returnvalue (`GameplayStatics.GetPlayerCharacter` 0))
  (`/Engine/EditorBlueprintResources/StandardMacros.IsValid` _returnvalue
    (:`Is Valid`
      (`SceneComponent.K2_SetWorldRotation` (`self.CapsuleComponent`) (`KismetMathLibrary.RInterpTo` (`SceneComponent.K2_GetComponentRotation` (`self.CapsuleComponent`)) (`KismetMathLibrary.FindLookAtRotation` (`SceneComponent.K2_GetComponentLocation` (`self.CapsuleComponent`)) (`self.K2_GetActorLocation` _returnvalue)) (`GameplayStatics.GetWorldDeltaSeconds`) 2.5) false false))))

(event `self.Box.OnComponentBeginOverlap`
  (params (OverlappedComponent :type "PrimitiveComponent Object Reference") (OtherActor :type "Actor Object Reference") (OtherComp :type "PrimitiveComponent Object Reference") (OtherBodyIndex :type Integer) (bFromSweep :type Boolean) (SweepResult :type "HitResult Structure (by ref)"))
  (if (== (`GameplayStatics.GetObjectClass` OtherActor) "/Game/Blueprints/BP_FirstPersonCharacter.BP_FirstPersonCharacter_C")
    (set `self.canShoot` true)
    (`self.StartShooting`)))

(event `self.Box.OnComponentEndOverlap`
  (params (OverlappedComponent :type "PrimitiveComponent Object Reference") (OtherActor :type "Actor Object Reference") (OtherComp :type "PrimitiveComponent Object Reference") (OtherBodyIndex :type Integer))
  (if (== (`GameplayStatics.GetObjectClass` OtherActor) "/Game/Blueprints/BP_FirstPersonCharacter.BP_FirstPersonCharacter_C")
    (set `self.canShoot` false)
    (`self.StartShooting`)))

(event `Danger`)

(event `self.Weakpoint.OnComponentBeginOverlap`
  (params (OverlappedComponent :type "PrimitiveComponent Object Reference") (OtherActor :type "Actor Object Reference") (OtherComp :type "PrimitiveComponent Object Reference") (OtherBodyIndex :type Integer) (bFromSweep :type Boolean) (SweepResult :type "HitResult Structure (by ref)"))
  (if (== (`GameplayStatics.GetObjectClass` OtherActor) "/Game/Blueprints/Enemies/DragonFly/BP_DragonFlyTest.BP_DragonFlyTest_C")
    (bind _asbp_dragon_fly_test (cast `/Game/Blueprints/Enemies/DragonFly/BP_DragonFlyTest` OtherActor))
    (if (`PrimitiveComponent.IsOverlappingComponent` (`self.Weakpoint`) (`/Game/Blueprints/Enemies/DragonFly/BP_DragonFlyTest.Collision` _asbp_dragon_fly_test))
      (`KismetSystemLibrary.DelayUntilNextTick`)
      (`KismetSystemLibrary.DelayUntilNextTick`)
      (`self.Kill Enemy`))))

(fn `Alert`
  (`parent.Alert`)
  (`self.StartShooting`)
  (`ActorComponent.K2_DestroyComponent` (`self.Box`)))

(fn `UserConstructionScript`
  (`parent.UserConstructionScript`))