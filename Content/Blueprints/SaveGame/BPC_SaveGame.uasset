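; Save component for the first-person player character that persists skill tree progress to a save slot.
; SaveGame writes points, active inner/outer skill pointers and each skill's own state into SG_SaveStats, reusing any existing save.
; LoadGame runs on BeginPlay, restores those values and calls OnSkillChanged, or creates a save when none exists.
; Events and debug keys trigger save, load and delete; another key prints every skill's status.
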(event Custom|SaveTheGame
  (CallFunction|SaveGame (Variables|Default|GetSlot%20Name%20Save))
  (Development|PrintString "Saved!"))

(event Custom|DeleteSave
  (SaveGame|DeleteGameinSlot (Variables|Default|GetSlot%20Name%20Save))
  (Development|PrintString "Deleted!"))

(event Custom|LoadTheLevel
  (CallFunction|LoadGame (Variables|Default|GetSlot%20Name%20Save)))

(event EventBeginPlay
  (Utilities|FlowControl|Sequence
    (:then_0
      (bind _asbp_first_person_character (Utilities|Casting|CastToBP_FirstPersonCharacter (Game|GetPlayerCharacter 0)))
      (Variables|Default|SetOwningCharacter _asbp_first_person_character))
    (:then_1
      (CallFunction|LoadGame (Variables|Default|GetSlot%20Name%20Save)))))

(event Input|KeyboardEvents|DebugKey1
  (params (Key :type Key%20Structure :default "None") (ActionValue :type Input%20Action%20Value%20Structure))
  (:Pressed
    (CallFunction|SaveGame (Variables|Default|GetSlot%20Name%20Save))
    (Development|PrintString "Saved!")))

(event Input|KeyboardEvents|DebugKey2
  (params (Key :type Key%20Structure :default "None") (ActionValue :type Input%20Action%20Value%20Structure))
  (:Pressed
    (SaveGame|DeleteGameinSlot (Variables|Default|GetSlot%20Name%20Save))
    (Development|PrintString "Deleted!")))

(event Input|KeyboardEvents|DebugKey3
  (params (Key :type Key%20Structure :default "None") (ActionValue :type Input%20Action%20Value%20Structure))
  (:Pressed
    (CallFunction|LoadGame (Variables|Default|GetSlot%20Name%20Save))))

(event Input|KeyboardEvents|DebugKey4
  (params (Key :type Key%20Structure :default "None") (ActionValue :type Input%20Action%20Value%20Structure))
  (bind _owningcharacter (Variables|Default|GetOwningCharacter))
  (bind _skilltreecomponent (Variables|/Game/Blueprints/BP_FirstPersonCharacter.BP_FirstPersonCharacter_C|GetSkillTreeComponent _owningcharacter))
  (:Pressed
    (bind _keys (Default|GetCategories _skilltreecomponent))
    (for _array_element _keys
      (bind (_value _found_) (Default|GetSkillArray _skilltreecomponent _array_element))
      (if _found_
        (for _array_element_2 (Utilities|Struct|BreakS_SkillArray _value)
          (Development|PrintString (Utilities|GetDisplayName _array_element_2))
          (Development|PrintString (Utilities|String|EnumtoString (Default|GetStatus _array_element_2)) true true "(R=1.000000,G=0.118751,B=0.000000,A=1.000000)"))))))

(fn SaveGame
  (params (SlotName :type String))
  (bind _owningcharacter (Variables|Default|GetOwningCharacter))
  (bind _owningcharacter_2 (Variables|Default|GetOwningCharacter))
  (bind _skilltreecomponent (Variables|/Game/Blueprints/BP_FirstPersonCharacter.BP_FirstPersonCharacter_C|GetSkillTreeComponent _owningcharacter_2))
  (bind _returnvalue (SaveGame|DoesSaveGameExist SlotName))
  (if _returnvalue
    (bind _returnvalue_2 (SaveGame|LoadGamefromSlot SlotName))
    (Variables|Default|SetSafe%20REF _returnvalue_2)
    (else
      (bind _returnvalue_3 (SaveGame|CreateSaveGameObject "/Game/Blueprints/SaveGame/SG_SaveStats.SG_SaveStats_C"))
      (bind _output_get (Variables|Default|SetSafe%20REF _returnvalue_3))))
  (bind _assg_save_stats (Utilities|Casting|CastToSG_SaveStats _output_get))
  (Variables|/Game/Blueprints/SaveGame/SG_SaveStats.SG_SaveStats_C|SetPoints _assg_save_stats (Variables|/Game/SkillTree/Component/SkillTreeComponent.SkillTreeComponent_C|GetPoints (Variables|/Game/Blueprints/BP_FirstPersonCharacter.BP_FirstPersonCharacter_C|GetSkillTreeComponent _owningcharacter)))
  (Variables|/Game/Blueprints/SaveGame/SG_SaveStats.SG_SaveStats_C|SetOuterPointerActive _assg_save_stats (Variables|/Game/Blueprints/BP_FirstPersonCharacter.BP_FirstPersonCharacter_C|GetOuterPointerSkills _owningcharacter))
  (Variables|/Game/Blueprints/SaveGame/SG_SaveStats.SG_SaveStats_C|SetInnerPointerActive _assg_save_stats (Variables|/Game/Blueprints/BP_FirstPersonCharacter.BP_FirstPersonCharacter_C|GetInnerPointerSkills _owningcharacter))
  (bind _keys (Default|GetCategories _skilltreecomponent))
  (for _array_element _keys
    (bind (_value _found_) (Default|GetSkillArray _skilltreecomponent _array_element))
    (if _found_
      (for _array_element_2 (Utilities|Struct|BreakS_SkillArray _value)
        (Development|PrintString "I AM WORKING")
        (Default|Save _array_element_2 _assg_save_stats))))
  (SaveGame|SaveGametoSlot _assg_save_stats SlotName)
  (Development|PrintString "DONE" true true "(R=0.307913,G=1.000000,B=0.000000,A=1.000000)"))

(fn LoadGame
  (params (SlotName :type String))
  (bind _owningcharacter (Variables|Default|GetOwningCharacter))
  (bind _returnvalue (SaveGame|DoesSaveGameExist SlotName))
  (if _returnvalue
    (bind _returnvalue_2 (SaveGame|LoadGamefromSlot SlotName))
    (bind _assg_save_stats (Utilities|Casting|CastToSG_SaveStats _returnvalue_2))
    (Variables|/Game/SkillTree/Component/SkillTreeComponent.SkillTreeComponent_C|SetPoints (Variables|/Game/Blueprints/BP_FirstPersonCharacter.BP_FirstPersonCharacter_C|GetSkillTreeComponent _owningcharacter) (Variables|/Game/Blueprints/SaveGame/SG_SaveStats.SG_SaveStats_C|GetPoints _assg_save_stats))
    (Variables|/Game/Blueprints/BP_FirstPersonCharacter.BP_FirstPersonCharacter_C|SetOuterPointerSkills _owningcharacter (Variables|/Game/Blueprints/SaveGame/SG_SaveStats.SG_SaveStats_C|GetOuterPointerActive _assg_save_stats))
    (Variables|/Game/Blueprints/BP_FirstPersonCharacter.BP_FirstPersonCharacter_C|SetInnerPointerSkills _owningcharacter (Variables|/Game/Blueprints/SaveGame/SG_SaveStats.SG_SaveStats_C|GetInnerPointerActive _assg_save_stats))
    (Default|OnSkillChanged (Variables|Default|GetOwningCharacter))
    (bind _keys (Utilities|Map|Keys (Variables|/Game/Blueprints/SaveGame/SG_SaveStats.SG_SaveStats_C|GetSkillStatusSaver _assg_save_stats)))
    (for _array_element _keys
      (if (Utilities|IsValid _array_element)
        (Default|Load _array_element _assg_save_stats)))
    (else
      (CallFunction|SaveGame SlotName))))