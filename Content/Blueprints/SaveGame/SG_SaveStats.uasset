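; SG_SaveStats is a save game Blueprint that holds skill statuses.
; It keeps them in the SkillStatusSaver map, keyed by skill.
; GetSkills returns the map's keys, and GetStatusses looks up the status stored for a given skill, returning it when the map contains that skill.
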(fn `GetSkills`
  (returns (Keys :type "Array of /Game/SkillTree/Skills/BP_Skill Object Reference"))
  (bind _keys (`BlueprintMapLibrary.Map_Keys` (`self.SkillStatusSaver`)))
  (return _keys))

(fn `GetStatusses`
  (params (Skill :type "/Game/SkillTree/Skills/BP_Skill Object Reference"))
  (returns (Value :type "/Game/SkillTree/E_SkillStatus Enum"))
  (if (`BlueprintMapLibrary.Map_Contains` (`self.SkillStatusSaver`) Skill)
    (return (`BlueprintMapLibrary.Map_Find` (`self.SkillStatusSaver`) (`local.Skill`)))))