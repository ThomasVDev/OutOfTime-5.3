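; Player health component that tracks hit points and handles taking damage.
; On BeginPlay it sets current health to the maximum.
; TakeDamage removes one point per hit and calls GetKnockback, which only plays a camera shake on the first player controller, or calls Die when health is at one.
; Die, Respawn, RegenerateHealth and SetCurrentHealth are empty stubs.
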(event `self.ReceiveBeginPlay`
  (`self.SetMaxHealth`))

(fn `Die`)

(fn `GetKnockback`
  (`PlayerController.ClientStartCameraShake` :`self` (`GameplayStatics.GetPlayerController` 0) :`Shake` "/Game/Blueprints/Headbobbing/CameraShake/TakeDamage.TakeDamage_C"))

(fn `RegenerateHealth`)

(fn `Respawn`)

(fn `SetCurrentHealth`)

(fn `SetMaxHealth`
  (set `self.PlayerHealth` (`self.MaxPlayerHealth`))
  (return))

(fn `TakeDamage`
  (if (== (`self.PlayerHealth`) 1)
    (`self.Die`)
    (else
      (bind _result (`/Engine/EditorBlueprintResources/StandardMacros.DecrementInt` (`self.PlayerHealth`))
        (:`  `
          (set `self.PlayerHealth` _result)
          (`self.GetKnockback`))))))