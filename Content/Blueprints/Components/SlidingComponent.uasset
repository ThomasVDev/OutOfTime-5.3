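; Sliding component that drives walking, sliding and crouching states on BP_FirstPersonCharacter, fetched as player 0.
; Tick derives a downhill vector from the floor normal by double cross product, feeding slide forces and braking.
; Slide entry boosts forward velocity and lowers friction; slow slides resolve to walking or crouching via slide-key and headroom checks.
; Helpers blend capsule and camera height and compute slope-based jump direction.
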(event `self.ReceiveBeginPlay`
  (bind _asbp_first_person_character (`self.GetPlayer`))
  (bind (_relativelocation_x _relativelocation_y _relativelocation_z) (`KismetMathLibrary.BreakVector` (`SceneComponent.RelativeLocation` (`/Game/Blueprints/BP_FirstPersonCharacter.FirstPersonCamera` _asbp_first_person_character))))
  (set `self.StandingCapsuleHeight` (`CapsuleComponent.GetScaledCapsuleHalfHeight` (`Character.CapsuleComponent` _asbp_first_person_character)))
  (set `self.StandingCameraZOffset` _relativelocation_z))

(event `self.ReceiveTick`
  (params (DeltaSeconds :type "Float (single-precision)"))
  (bind (_currentfloor_bblockinghit _currentfloor_bwalkablefloor _currentfloor_blinetrace _currentfloor_floordist _currentfloor_linedist _currentfloor_hitresult) (break `FindFloorResult` (`CharacterMovementComponent.CurrentFloor` (`Character.CharacterMovement` (`self.GetPlayer`)))))
  (bind _return_value (`self.CalculateFloorInfluence` (`.Normal` (`GameplayStatics.BreakHitResult` _currentfloor_hitresult))))
  (set `self.FloorNormalInfluence` _return_value))

(fn `CalculateFloorInfluence`
  (params (FloorNormal :type "Vector Structure"))
  (returns (`Return Value` :type "Vector Structure"))
  (bind _floornormal (`local.FloorNormal`))
  (if (== FloorNormal (`KismetMathLibrary.Vector_Up`) :`ErrorTolerance` 0.0001)
    (set `self.BDW_WhileSliding` 1000.0)
    (return (0.0 0.0 0.0))
    (else
      (set `self.BDW_WhileSliding` 0.0)
      (return (* (* (`KismetMathLibrary.Normal` (`KismetMathLibrary.Cross_VectorVector` _floornormal (`KismetMathLibrary.Cross_VectorVector` _floornormal (`KismetMathLibrary.Vector_Up`)))) (* (`KismetMathLibrary.FClamp` (- 1.0 (`KismetMathLibrary.Dot_VectorVector` (`local.FloorNormal`) (`KismetMathLibrary.Vector_Up`)))) 50.0)) (`self.FloorInfluenceMultiplier`))))))

(fn `CanStand`
  (returns (Result :type Boolean))
  (bind _asbp_first_person_character (`self.GetPlayer`))
  (bind _returnvalue (- (`Actor.K2_GetActorLocation` _asbp_first_person_character) (`KismetMathLibrary.MakeVector` 0.0 0.0 (`CapsuleComponent.GetScaledCapsuleHalfHeight` (`Character.CapsuleComponent` _asbp_first_person_character)))))
  (if (`self.SlideKeyDown?`)
    (return false)
    (else
      (bind (_outhit _returnvalue_2) (`KismetSystemLibrary.LineTraceSingle` _returnvalue (+ _returnvalue (`KismetMathLibrary.MakeVector` 0.0 0.0 (* (`self.StandingCapsuleHeight`) 2.0))) "TraceTypeQuery1"))
      (return (not _returnvalue_2)))))

(fn `GetPlayer`
  (returns (`AsBP First Person Character` :type "/Game/Blueprints/BP_FirstPersonCharacter Object Reference"))
  (return (cast `/Game/Blueprints/BP_FirstPersonCharacter` (`GameplayStatics.GetPlayerCharacter` 0) :!pure true)))

(fn `JumpBasedOnFloorAngleAndSpeed`
  (returns (JumpDirection :type "Vector Structure") (NeedsDirection :type Boolean))
  (bind _asbp_first_person_character (`self.GetPlayer`))
  (bind (_currentfloor_bblockinghit _currentfloor_bwalkablefloor _currentfloor_blinetrace _currentfloor_floordist _currentfloor_linedist _currentfloor_hitresult) (break `FindFloorResult` (`CharacterMovementComponent.CurrentFloor` (`Character.CharacterMovement` (`self.GetPlayer`)))))
  (bind (_bblockinghit _binitialoverlap _time _distance _location _impactpoint _normal) (`GameplayStatics.BreakHitResult` _currentfloor_hitresult))
  (bind _returnvalue (/ (`CharacterMovementComponent.MaxWalkSpeed` (`Character.CharacterMovement` _asbp_first_person_character)) (`self.SlideJumpDivider`)))
  (if (== _normal (0.0 0.0 1.0) :`ErrorTolerance` 1e-05)
    (return (0.0 0.0 0.0) false)
    (else
      (return (+ (* (* _normal (`self.FloorNormalMultiplier`)) _returnvalue) (* (`KismetMathLibrary.GetForwardVector` (`SceneComponent.K2_GetComponentRotation` (`Character.CapsuleComponent` _asbp_first_person_character))) _returnvalue)) true))))

(fn `On Movement State Changed`
  (params (PrevMovementState :type "/Game/Blueprints/Enums/E_MovementState Enum" :default "NewEnumerator0"))
  (bind _asbp_first_person_character (`self.GetPlayer`))
  (bind _asbp_first_person_character_2 (`self.GetPlayer`))
  (bind _asbp_first_person_character_3 (`self.GetPlayer`))
  (bind _charactermovement (`Character.CharacterMovement` _asbp_first_person_character))
  (bind _charactermovement_2 (`Character.CharacterMovement` _asbp_first_person_character_2))
  (`|ExecutionSequence`
    (:`then_0`
      ;[0.6929 0.6079 1 0.251] Set Walk speeds for change in movement speed that Isnt sliding
      (set `CharacterMovementComponent.MaxWalkSpeed` (select `/Game/Blueprints/Enums/E_MovementState` (`self.MovementState`) :`NewEnumerator0` (`/Game/Blueprints/BP_FirstPersonCharacter.Def_WalkSpeed` _asbp_first_person_character_3) :`NewEnumerator2` (`/Game/Blueprints/BP_FirstPersonCharacter.Def_CrouchSpeed` _asbp_first_person_character_3) :!type "Float (single-precision)") (`Character.CharacterMovement` (`self.GetPlayer`))))
    (:`then_1`
      ;[0 1 0.7243 0.429] If Previous movement state was Sliding
      (switch `/Game/Blueprints/Enums/E_MovementState` (`local.PrevMovementState`)
        (:`NewEnumerator1`
          (set `CharacterMovementComponent.GroundFriction` (`/Game/Blueprints/BP_FirstPersonCharacter.Def_GroundFriction` _asbp_first_person_character_2) _charactermovement_2)
          (set `CharacterMovementComponent.BrakingDecelerationWalking` (`/Game/Blueprints/BP_FirstPersonCharacter.Def_BrakingDecelerationWalking` _asbp_first_person_character_2) _charactermovement_2)
          (`/Game/Blueprints/BP_FirstPersonCharacter.EndSlide` (`self.GetPlayer`)))))
    (:`then_2`
      ;[1 0.8799 0.1248 0.445] If New movement state is Sliding
      (`self.StateMovement`
        (:`Sliding`
          (bind _output_get (set `self.SlideAfterCalcsVelocity` (+ (`self.SlideVelocity`) (* (`CharacterMovementComponent.MaxWalkSpeed` _charactermovement) 8.0))))
          (bind _output_get_2 (set `MovementComponent.Velocity` (* (`Actor.GetActorForwardVector` _asbp_first_person_character) _output_get) _charactermovement))
          (`CharacterMovementComponent.AddForce` _charactermovement _output_get_2)
          (set `CharacterMovementComponent.GroundFriction` 0.5 _charactermovement)
          (if (== (`self.FloorNormalInfluence`) (0.0 0.0 0.0) :`ErrorTolerance` 1e-05)
            (set `CharacterMovementComponent.BrakingDecelerationWalking` 1000.0 _charactermovement)
            (else
              (set `CharacterMovementComponent.BrakingDecelerationWalking` 0.0 _charactermovement))))))))

(fn `ResolveMovement`
  (`self.SetMovementState` (select `bool` (`self.CanStand`) :`false` "NewEnumerator2" :`true` "NewEnumerator0" :!type "/Game/Blueprints/Enums/E_MovementState Enum")))

(fn `SetCapsuleHeight`
  (params (HalfHeight :type "Float (double-precision)"))
  (bind _asbp_first_person_character (`self.GetPlayer`))
  (bind _firstpersoncamera (`/Game/Blueprints/BP_FirstPersonCharacter.FirstPersonCamera` _asbp_first_person_character))
  (bind (_relativelocation_x _relativelocation_y) (`KismetMathLibrary.BreakVector` (`SceneComponent.RelativeLocation` _firstpersoncamera)))
  (`CapsuleComponent.SetCapsuleHalfHeight` (`Character.CapsuleComponent` _asbp_first_person_character) (`KismetMathLibrary.MapRangeClamped` HalfHeight 0.0 1.0 35.0 (`self.StandingCapsuleHeight`)) true)
  (`SceneComponent.K2_SetRelativeLocation` _firstpersoncamera (`KismetMathLibrary.MakeVector` _relativelocation_x _relativelocation_y (`KismetMathLibrary.MapRangeClamped` HalfHeight 0.0 1.0 25.0 (`self.StandingCameraZOffset`))) false false))

(fn `SetMovementState`
  (params (NewMovementState :type "/Game/Blueprints/Enums/E_MovementState Enum" :default "NewEnumerator0"))
  (locals (`Prev MovementState (Local)` :type "/Game/Blueprints/Enums/E_MovementState Enum"))
  (bind _asbp_first_person_character (`self.GetPlayer`))
  (if (`|EnumInequality` NewMovementState (`self.MovementState`))
    (set `local.Prev MovementState (Local)` (`self.MovementState`))
    (set `self.MovementState` (`local.NewMovementState`))
    (`self.On Movement State Changed` (`local.Prev MovementState (Local)`))
    (`self.StateMovement`
      (:`Walking`
        (`/Game/Blueprints/BP_FirstPersonCharacter.EndCrouch` _asbp_first_person_character))
      (:`Sliding`
        (`/Game/Blueprints/BP_FirstPersonCharacter.BeginCrouch` _asbp_first_person_character)
        (`/Game/Blueprints/BP_FirstPersonCharacter.BeginSlide` _asbp_first_person_character))
      (:`Crouching`
        (`/Game/Blueprints/BP_FirstPersonCharacter.BeginCrouch` _asbp_first_person_character)))))

(fn `SetSlideVelocityWithAngleForce`
  (bind _asbp_first_person_character (`self.GetPlayer`))
  (bind _asbp_first_person_character_2 (`self.GetPlayer`))
  (bind _asbp_first_person_character_3 (`self.GetPlayer`))
  (`CharacterMovementComponent.AddForce` (`Character.CharacterMovement` _asbp_first_person_character_2) (* (* (`self.FloorNormalInfluence`) 2.0) (* (`/Game/Blueprints/BP_FirstPersonCharacter.MaxSpeeding` _asbp_first_person_character_2) 2.0)))
  (`|ExecutionSequence`
    (:`then_0`
      (set `MovementComponent.Velocity` (* (`KismetMathLibrary.Normal` (`Actor.GetVelocity` _asbp_first_person_character)) (* (`self.SlideAfterCalcsVelocity`) 2.0)) (`Character.CharacterMovement` _asbp_first_person_character)))
    (:`then_1`
      (if (<= (`KismetMathLibrary.VSize` (`Actor.GetVelocity` _asbp_first_person_character_3)) (`/Game/Blueprints/BP_FirstPersonCharacter.Def_CrouchSpeed` _asbp_first_person_character_3))
        (`self.ResolveMovement`)))))

(fn `UpdateSlide`
  (params (Growth :type "Float (double-precision)"))
  (bind _asbp_first_person_character (`self.GetPlayer`))
  (bind _asbp_first_person_character_2 (`self.GetPlayer`))
  (bind _asbp_first_person_character_3 (`self.GetPlayer`))
  (`CharacterMovementComponent.AddForce` (`Character.CharacterMovement` _asbp_first_person_character_2) (* (* (`self.FloorNormalInfluence`) Growth) (* (`/Game/Blueprints/BP_FirstPersonCharacter.MaxSpeeding` _asbp_first_person_character_2) 2.0)))
  (`|ExecutionSequence`
    (:`then_0`
      (set `MovementComponent.Velocity` (* (`KismetMathLibrary.Normal` (`Actor.GetVelocity` _asbp_first_person_character)) (* (`self.SlideAfterCalcsVelocity`) (`local.Growth`))) (`Character.CharacterMovement` _asbp_first_person_character)))
    (:`then_1`
      (if (<= (`KismetMathLibrary.VSize` (`Actor.GetVelocity` _asbp_first_person_character_3)) (`/Game/Blueprints/BP_FirstPersonCharacter.Def_CrouchSpeed` _asbp_first_person_character_3))
        (`self.ResolveMovement`)))))