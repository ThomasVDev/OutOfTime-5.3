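; Player skating component that slides the first-person character along BP_SlideRamp actors.
; CheckForSkate line-traces below the capsule, enters the skating state on a ramp hit, then calls the stored ramp's RotateCamera.
; While skating, Tick zeroes friction, cuts camera sensitivity and forces a fixed-speed velocity along the ramp's CameraLookAt forward vector.
; Otherwise it restores default friction and sensitivity each tick; leaving the skating state relies on SetIsSkating.
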(event `self.ReceiveBeginPlay`
  (bind _asbp_first_person_character (cast `/Game/Blueprints/BP_FirstPersonCharacter` (`GameplayStatics.GetPlayerCharacter` 0)))
  (bind _output_get (set `self.OwningCharacter` _asbp_first_person_character))
  (set `self.OwningMovement` (`Character.CharacterMovement` _output_get))
  (set `self.E_IsSkating?` "NewEnumerator0"))

(event `self.ReceiveTick`
  (params (DeltaSeconds :type "Float (single-precision)"))
  (bind _owningmovement (`self.OwningMovement`))
  (bind _owningcharacter (`self.OwningCharacter`))
  (switch `/Game/Blueprints/Enums/E_isSkating` (`self.E_IsSkating?`)
    (:`NewEnumerator0`
      (`/Game/Blueprints/BP_FirstPersonCharacter.SetCameraSens` (`self.OwningCharacter`) 1.0)
      (set `CharacterMovementComponent.BrakingFriction` (`/Game/Blueprints/BP_FirstPersonCharacter.Def_BrakingFriction` _owningcharacter) _owningmovement)
      (set `CharacterMovementComponent.GroundFriction` (`/Game/Blueprints/BP_FirstPersonCharacter.Def_GroundFriction` _owningcharacter) _owningmovement))
    (:`NewEnumerator1`
      (`self.CalculateFloorAngles` (0.0 0.0 0.0)))))

(event `CheckForSkate`
  (`self.CheckForSkateFloor`)
  (`self.Camera Look At`))

(fn `CalculateFloorAngles`
  (params (Direction :type "Vector Structure"))
  (locals (`Current Rot` :type "Rotator Structure") (End :type "Float (double-precision)") (Durations :type "Float (double-precision)") (`Time Of Active` :type "Float (double-precision)"))
  (bind _owningmovement (`self.OwningMovement`))
  (set `local.Current Rot` (`SceneComponent.K2_GetComponentRotation` (`/Game/Blueprints/BP_FirstPersonCharacter.FirstPersonCamera` (`self.OwningCharacter`))))
  (set `CharacterMovementComponent.BrakingFriction` 0.0 _owningmovement)
  (set `CharacterMovementComponent.GroundFriction` 0.0 _owningmovement)
  (set `MovementComponent.Velocity` (* (`SceneComponent.GetForwardVector` (`/Game/Blueprints/PlayerUse/BP_SlideRamp.CameraLookAt` (`self.CurrentSlideRamp`))) 3000.0) (`self.OwningMovement`))
  (`/Game/Blueprints/BP_FirstPersonCharacter.SetCameraSens` (`self.OwningCharacter`) 0.1))

(fn `Camera Look At`
  (`/Game/Blueprints/PlayerUse/BP_SlideRamp.RotateCamera` (`self.CurrentSlideRamp`))
  (return))

(fn `CheckFloor`
  (returns (ReturnValue :type Boolean) (OutHit :type "HitResult Structure"))
  (bind _returnvalue (`SceneComponent.K2_GetComponentLocation` (`Character.CapsuleComponent` (`self.OwningCharacter`))))
  (bind (_outhit _returnvalue_2) (`KismetSystemLibrary.LineTraceSingle` :`Start` _returnvalue :`End` (`KismetMathLibrary.MakeVector` (.x _returnvalue) (.y _returnvalue) (- (.z _returnvalue) 120.0)) :`TraceChannel` "TraceTypeQuery1" :`DrawDebugType` "ForDuration"))
  (return _returnvalue_2 _outhit))

(fn `CheckForSkateFloor`
  (returns (OutputPin :type "Vector Structure"))
  (locals (TimeOfActivation :type "Float (double-precision)") (DurationOfRotation :type "Float (double-precision)" :default 0.5))
  (set `local.TimeOfActivation` (`GameplayStatics.GetRealTimeSeconds`))
  (bind (_returnvalue _outhit) (`self.CheckFloor`))
  (if _returnvalue
    (bind (_bblockinghit _binitialoverlap _time _distance _location _impactpoint _normal _impactnormal _physmat _hitactor) (`GameplayStatics.BreakHitResult` _outhit))
    (if (== (`GameplayStatics.GetObjectClass` _hitactor) "/Game/Blueprints/PlayerUse/BP_SlideRamp.BP_SlideRamp_C")
      (bind _asbp_slide_ramp (cast `/Game/Blueprints/PlayerUse/BP_SlideRamp` _hitactor))
      (set `self.CurrentSlideRamp` _asbp_slide_ramp)
      (`/Game/Blueprints/BP_FirstPersonCharacter.SetCurrentPlayerAction` (`self.OwningCharacter`) "NewEnumerator4")
      (set `self.E_IsSkating?` "NewEnumerator1")
      (return _impactnormal))))

(fn `GetIsSkating`
  (returns (`E_IsSkating?` :type "/Game/Blueprints/Enums/E_isSkating Enum"))
  (return (`self.E_IsSkating?`)))

(fn `SetIsSkating`
  (params (IsSkating :type "/Game/Blueprints/Enums/E_isSkating Enum" :default "NewEnumerator0"))
  (set `self.E_IsSkating?` IsSkating)
  (return))

(fn `SetMovementModeChanged`)