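; Actor component that lets BP_FirstPersonCharacter vault onto ledges.
; While not vaulting, each tick traces down ahead of the capsule and validates height, walkable slope and capsule clearance, caching the landing point, which a failed check leaves uncleared.
; The Vault event starts a timed lerp to that point, teleporting the character without sweep.
; Completion clears the point and adds to MaxWalkSpeed, with no reset in this component.
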(event `self.ReceiveBeginPlay`
  ;[1 1 1 0.293] Set Owning character as BP_FPC
  (bind _asbp_first_person_character (cast `/Game/Blueprints/BP_FirstPersonCharacter` (`self.GetOwner`)))
  (set `self.OwningCharacter` _asbp_first_person_character))

(event `self.ReceiveTick`
  (params (DeltaSeconds :type "Float (single-precision)"))
  ;[1 0.5521 0.5521 0.419] Am I vaulting Yes or No? If yes, Vault. If no, Check if I can Vault
  (`self.SwitchVaultingState`
    (:`NotVaulting`
      (bind (_result _endinglocation) (`self.CanVault`))
      (if _result
        (set `self.Ending Location` _endinglocation)
        (else
          (set `self.Vaulting?` false))))
    (:`Vaulting`
      (`self.TickVault` DeltaSeconds)
      (set `self.Vaulting?` true))))

(event `Vault`
  ;[1 0.6005 0.2592 0.414] Start at 0, then switch to vaulting
  (if (not (== (`self.Ending Location`) (0.0 0.0 0.0)))
    (set `self.Progress` 0.0)
    (set `self.Starting Location` (`Actor.K2_GetActorLocation` (`self.OwningCharacter`)))
    (set `self.VaultingState` "NewEnumerator1")))

(fn `CanVault`
  (returns (Result :type Boolean) (EndingLocation :type "Vector Structure"))
  (locals (`Capsule (Local)` :type "CapsuleComponent Object Reference") (DistanceForwardChecker :type "Float (double-precision)" :default 60.0))
  (bind _returnvalue (`CapsuleComponent.GetScaledCapsuleHalfHeight` (`local.Capsule (Local)`)))
  (bind _capsulecomponent (`Character.CapsuleComponent` (`self.OwningCharacter`)))
  (bind _returnvalue_2 (+ (`SceneComponent.K2_GetComponentLocation` _capsulecomponent) (* (`SceneComponent.GetForwardVector` _capsulecomponent) (`local.DistanceForwardChecker`))))
  ;[0.4855 0.8167 1 0.675] If Im NOT vaulting
  (if (`|EnumEquality` (`self.VaultingState`) "NewEnumerator0")
    (set `local.Capsule (Local)` (`Character.CapsuleComponent` (`self.OwningCharacter`)))
    ;[0.08348 0.224 0.1408 0.791] Did I hit yes or no? If yes, where and what location?
    (bind (_outhit _returnvalue_3) (`KismetSystemLibrary.LineTraceSingle` (+ _returnvalue_2 (`KismetMathLibrary.MakeVector` 0.0 0.0 (+ _returnvalue (`self.MaxVaultingHeight`)))) (- _returnvalue_2 (`KismetMathLibrary.MakeVector` 0.0 0.0 (+ _returnvalue 0.0))) "TraceTypeQuery1" false (`|MakeArray` (`self.OwningCharacter`) :!type "Actor Object Reference") "None" true (struct :`R` 1.0 :`A` 1.0) (struct :`G` 1.0 :`A` 1.0) 2.0))
    (if _returnvalue_3
      (bind (_result _endinglocation) (`self.CanVaultToHit` (`local.Capsule (Local)`) _outhit))
      (return _result _endinglocation)
      (else
        (return false (0.0 0.0 0.0))))
    (else
      (return false (0.0 0.0 0.0)))))

(fn `CanVaultToHit`
  (params (Capsule :type "CapsuleComponent Object Reference") (Hit :type "HitResult Structure"))
  (returns (Result :type Boolean) (EndingLocation :type "Vector Structure"))
  (locals (`EndingLocation(Local)` :type "Vector Structure" :default (0.0 0.0 0.0)))
  (bind (_hit_bblockinghit _hit_binitialoverlap _hit_time _hit_distance _hit_location _hit_impactpoint _hit_normal _hit_impactnormal _hit_physmat _hit_hitactor _hit_hitcomponent _hit_hitbonename _hit_bonename _hit_hititem _hit_elementindex _hit_faceindex _hit_tracestart _hit_traceend) (`GameplayStatics.BreakHitResult` (`local.Hit`)))
  (bind _capsule (`local.Capsule`))
  (bind (_hit_bblockinghit_2 _hit_binitialoverlap_2 _hit_time_2 _hit_distance_2 _hit_location_2 _hit_impactpoint_2 _hit_normal_2) (`GameplayStatics.BreakHitResult` (`local.Hit`)))
  (bind (_hit_bblockinghit_3 _hit_binitialoverlap_3 _hit_time_3 _hit_distance_3 _hit_location_3 _hit_impactpoint_3) (`GameplayStatics.BreakHitResult` (`local.Hit`)))
  (bind _returnvalue (`CapsuleComponent.GetScaledCapsuleRadius` _capsule))
  (`|ExecutionSequence`
    (:`then_0`
      ;[0.01562 0.01562 0.01562] appropiate height ledge check
      (if (not (`KismetMathLibrary.InRange_FloatFloat` (- (.z _hit_location) (.z _hit_traceend)) (`self.MinVaultingHeight`) (+ (`self.MaxVaultingHeight`) 1000.0)))
        (return false (0.0 0.0 0.0))))
    (:`then_1`
      ;[0.2188 0.2188 0.2188] Surface = in range and not steep
      (if (< (.z _hit_normal_2) (`CharacterMovementComponent.K2_GetWalkableFloorZ` (`Character.CharacterMovement` (`self.OwningCharacter`))))
        (return false (0.0 0.0 0.0))))
    (:`then_2`
      ;[1 1 1] Enough room for us
      (bind _output_get (set `local.EndingLocation(Local)` (+ _hit_impactpoint_3 (`KismetMathLibrary.MakeVector` 0.0 0.0 (`CapsuleComponent.GetScaledCapsuleHalfHeight` (`local.Capsule`))))))
      (bind _result (`self.CheckCapsuleCollision` (+ _output_get (`KismetMathLibrary.MakeVector` 0.0 0.0 _returnvalue)) (`CapsuleComponent.GetScaledCapsuleHalfHeight` _capsule) _returnvalue true))
      (if _result
        (return false (0.0 0.0 0.0))))
    (:`then_3`
      (return true (`local.EndingLocation(Local)`)))))

(fn `CheckCapsuleCollision`
  (params (Center :type "Vector Structure") (HalfHeight :type "Float (double-precision)") (Radius :type "Float (double-precision)") (DrawDebug :type Boolean))
  (returns (Result :type Boolean))
  (bind (_outactors _returnvalue) (`KismetSystemLibrary.CapsuleOverlapActors` (`local.Center`) (`local.Radius`) (`local.HalfHeight`) (`|MakeArray` "ObjectTypeQuery1" "ObjectTypeQuery2" "ObjectTypeQuery4" "ObjectTypeQuery5" "ObjectTypeQuery6" :!type "EObjectTypeQuery Enum") "/Script/Engine.Actor" (`|MakeArray` (`self.OwningCharacter`) :!type "Actor Object Reference")))
  (return _returnvalue))

(fn `TickVault`
  (params (DeltaSeconds :type "Float (double-precision)"))
  (bind _charactermovement (`Character.CharacterMovement` (`self.OwningCharacter`)))
  (`|ExecutionSequence`
    (:`then_0`
      ;[0.09837 0.3942 1 0.707] VAULTING
      (set `self.Progress` (`KismetMathLibrary.FClamp` (+ (`self.Progress`) (/ (`local.DeltaSeconds`) (`self.VaultSpeed`)))))
      (`Actor.K2_SetActorLocation` (`self.OwningCharacter`) (`KismetMathLibrary.VLerp` (`self.Starting Location`) (`self.Ending Location`) (`self.Progress`)) false true))
    (:`then_1`
      ;[0.3001 0.1914 1 0.361] After vaulting
      (if (>= (`self.Progress`) 1.0)
        (set `self.VaultingState` "NewEnumerator0")
        (set `CharacterMovementComponent.MaxWalkSpeed` (+ (`CharacterMovementComponent.MaxWalkSpeed` _charactermovement) 500.0) _charactermovement)
        (set `self.Ending Location` (0.0 0.0 0.0))))))