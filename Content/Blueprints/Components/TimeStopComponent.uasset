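; Player component for the time stop ability, which slows the world while compensating the character's own time dilation and desaturates through a material parameter collection.
; Tick drives a state enum that ramps dilation down, drains the meter, or recharges it toward a reuse threshold.
; While inactive, a camera trace finds BP_TimeStopTP targets, switching the input from slowdown to character teleport.
; The same press also launches toward the thrown sword when grappling is available.
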(event `self.ReceiveBeginPlay`
  (bind _asbp_first_person_character (cast `/Game/Blueprints/BP_FirstPersonCharacter` (`GameplayStatics.GetPlayerCharacter` 0)))
  (set `self.OwnerCharacter` _asbp_first_person_character)
  (set `self.E Time Stop Active` "NewEnumerator0")
  (set `self.TimeStopDuration` (`self.MaxTimeStopDuration`)))

(event `InputAction|TimeStop`
  (params (Key :type "Key Structure"))
  (:`Pressed`
    (switch `/Game/Blueprints/Enums/E_TimeStopUsable` (`self.E TimeStopUsable`)
      (:`NewEnumerator0`
        (`self.ActivateTimeStop`
          (:`Normal Time Stop`
            (set `self.E Time Stop Active` "NewEnumerator2"))
          (:`TP Time Stop`
            (`/Game/Blueprints/BP_FirstPersonCharacter.TimeStopTp` (`self.OwnerCharacter`)))
          (:`CanGrapple`
            (`/Game/Blueprints/Components/SwordThrowComponent.Launch Towards Sword` (`/Game/Blueprints/BP_FirstPersonCharacter.SwordThrowComponent` (`self.OwnerCharacter`))))))))
  (:`Released`
    (switch `/Game/Blueprints/Enums/E_TimeStopActive` (`self.E Time Stop Active`)
      (:`NewEnumerator1`
        _)
      (:`NewEnumerator2`
        _))
    (`self.End TimeStop`)))

(event `self.ReceiveTick`
  (params (DeltaSeconds :type "Float (single-precision)"))
  (switch `/Game/Blueprints/Enums/E_TimeStopActive` (`self.E Time Stop Active`)
    (:`NewEnumerator0`
      (`self.RechargeTimeStop`)
      (bind _tp_location (`self.WhatKindOfTimeStop?`))
      (set `self.TP Location` _tp_location)
      (`/Game/Blueprints/BP_FirstPersonCharacter.SetDashStrength` (`self.OwnerCharacter`) 1500.0))
    (:`NewEnumerator1`
      (`self.TimeStop Duration`))
    (:`NewEnumerator2`
      (`self.Normal Time Stop`))))

(fn `End TimeStop`
  (`GameplayStatics.SetGlobalTimeDilation` 1.0)
  (set `Actor.CustomTimeDilation` 1.0 (`self.OwnerCharacter`))
  (set `self.E Time Stop Active` "NewEnumerator0")
  (set `self.E TimeStopUsable` "NewEnumerator1")
  (`KismetMaterialLibrary.SetScalarParameterValue` "/Game/VFX/MPC_PlayerPosition.MPC_PlayerPosition" "Desaturation"))

(fn `GetMaxTimeStopDuration`
  (returns (MaxTimeStopDuration :type "Float (double-precision)"))
  (return (`self.MaxTimeStopDuration`)))

(fn `GetTimeStopActive`
  (returns (`E Time Stop Active` :type "/Game/Blueprints/Enums/E_TimeStopActive Enum"))
  (return (`self.E Time Stop Active`)))

(fn `GetTimeStopDuration`
  (returns (TimeStopDuration :type "Float (double-precision)"))
  (return (`self.TimeStopDuration`)))

(fn `Normal Time Stop`
  (locals (TimeDilation :type "Float (double-precision)" :default 0.0001))
  (bind _returnvalue (`GameplayStatics.GetGlobalTimeDilation`))
  (`/Game/Blueprints/BP_FirstPersonCharacter.SetDashStrength` (`self.OwnerCharacter`) (`self.DashStrength`))
  (`GameplayStatics.SetGlobalTimeDilation` (* _returnvalue 0.1))
  (set `Actor.CustomTimeDilation` (/ 1.0 _returnvalue) (`self.OwnerCharacter`))
  (if (<= (`GameplayStatics.GetGlobalTimeDilation`) (`local.TimeDilation`))
    (set `self.E Time Stop Active` "NewEnumerator1")
    (`KismetMaterialLibrary.SetScalarParameterValue` "/Game/VFX/MPC_PlayerPosition.MPC_PlayerPosition" "Desaturation" 1.0)))

(fn `RechargeTimeStop`
  (if (>= (`self.TimeStopDuration`) (`self.MaxTimeStopDuration`))
    (set `self.TimeStopDuration` (`self.MaxTimeStopDuration`))
    (else
      (bind _output_get (set `self.TimeStopDuration` (+ (`self.TimeStopDuration`) (`self.RechargeRate`))))
      (if (>= _output_get (* (`self.MaxTimeStopDuration`) 0.25))
        (set `self.E TimeStopUsable` "NewEnumerator0")))))

(fn `SetTimeStopDuration`
  (params (`DetractFromTS Duration` :type "Float (double-precision)"))
  (set `self.TimeStopDuration` (- (`self.TimeStopDuration`) `DetractFromTS Duration`))
  (return))

(fn `SPECIAL_ResumeTimeIndefinetly`)

(fn `SPECIAL_StopTimeIndefinetly`
  (params (PlayerDilation :type "Float (double-precision)"))
  (set `self.E Time Stop Active` "NewEnumerator3")
  (`GameplayStatics.SetGlobalTimeDilation` 0.0001)
  (set `Actor.CustomTimeDilation` (/ PlayerDilation (`GameplayStatics.GetGlobalTimeDilation`)) (`self.OwnerCharacter`))
  (`KismetMaterialLibrary.SetScalarParameterValue` "/Game/VFX/MPC_PlayerPosition.MPC_PlayerPosition" "Desaturation" 1.0)
  (return))

(fn `SprintBoostCombo`)

(fn `Time Stop TP`
  (params (`TP Location` :type "Vector Structure"))
  (`SceneComponent.K2_SetWorldLocation` (`Character.CapsuleComponent` (`self.OwnerCharacter`)) `TP Location` false true)
  (set `self.TimeStopDuration` 0.0))

(fn `TimeStop Duration`
  (set `self.TimeStopDuration` (- (`self.TimeStopDuration`) (`self.DepletionRate`)))
  (if (<= (`self.TimeStopDuration`) 0.0)
    (`self.End TimeStop`)))

(fn `WhatKindOfTimeStop?`
  (returns (`TP Location` :type "Vector Structure"))
  (locals (`Item To TP to` :type "/Game/Blueprints/PlayerUse/BP_TimeStopTP Object Reference") (HitActor :type "Actor Object Reference"))
  (bind _firstpersoncamera (`/Game/Blueprints/BP_FirstPersonCharacter.FirstPersonCamera` (`self.OwnerCharacter`)))
  (bind _returnvalue (`SceneComponent.K2_GetComponentLocation` _firstpersoncamera))
  (bind (_outhit _returnvalue_2) (`KismetSystemLibrary.LineTraceSingle` _returnvalue (+ _returnvalue (* (`KismetMathLibrary.GetForwardVector` (`SceneComponent.K2_GetComponentRotation` _firstpersoncamera)) (`self.TimeStopSightRange`))) "TraceTypeQuery1"))
  (if _returnvalue_2
    (bind _output_get (set `local.HitActor` (`.HitActor` (`GameplayStatics.BreakHitResult` _outhit))))
    (if (== (`GameplayStatics.GetObjectClass` _output_get) "/Game/Blueprints/PlayerUse/BP_TimeStopTP.BP_TimeStopTP_C")
      (bind _asbp_time_stop_tp (cast `/Game/Blueprints/PlayerUse/BP_TimeStopTP` (`local.HitActor`)))
      (bind _output_get_2 (set `local.Item To TP to` _asbp_time_stop_tp))
      (`/Game/Blueprints/PlayerUse/BP_TimeStopTP.Activated` _output_get_2)
      (set `self.E Time Stop Version` "NewEnumerator1")
      (return (`Actor.K2_GetActorLocation` (`local.HitActor`)))
      (else
        (set `self.E Time Stop Version` "NewEnumerator0")))
    (else
      (set `self.E Time Stop Version` "NewEnumerator0")
      (bind _outactors (`GameplayStatics.GetAllActorsOfClass` "/Game/Blueprints/PlayerUse/BP_TimeStopTP.BP_TimeStopTP_C"))
      (if (`KismetArrayLibrary.Array_IsValidIndex` _outactors)
        (for _array_element _outactors
          (`/Game/Blueprints/PlayerUse/BP_TimeStopTP.Deactivated` _array_element))))))