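; Wallrun component that supplies surface, direction and jump-off math for the first-person character, enabling its movement plane constraint on BeginPlay.
; Surfaces qualify by comparing their tilt against the walkable floor angle.
; Wall side comes from the normal against the player's right vector, then a cross product yields run direction.
; Launch velocity combines wall-away or airborne input direction, camera forward and height, scaled by walk speed and jump velocity.
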(event `self.ReceiveBeginPlay`
  (bind _asbp_first_person_character (`self.GetPlayer`))
  (`/Game/Blueprints/BP_FirstPersonCharacter.ResetJump` _asbp_first_person_character 0)
  (`MovementComponent.SetPlaneConstraintEnabled` (`Character.CharacterMovement` _asbp_first_person_character) true))

(fn `CanSurfaceBeWallrun`
  (params (SurfaceNormal :type "Vector Structure"))
  (returns (CanItBeWallrun :type Boolean))
  (if (< (.z SurfaceNormal) -0.05)
    (return false)
    (else
      (return (< (`KismetMathLibrary.DegAcos` (`KismetMathLibrary.Dot_VectorVector` (`KismetMathLibrary.Normal` (`KismetMathLibrary.MakeVector` (.x SurfaceNormal) (.y SurfaceNormal))) SurfaceNormal)) (`CharacterMovementComponent.K2_GetWalkableFloorAngle` (`Character.CharacterMovement` (`GameplayStatics.GetPlayerCharacter` 0))))))))

(fn `FindLaunchDirection`
  (returns (LaunchVelocity :type "Vector Structure"))
  (locals (LaunchDirection :type "Vector Structure"))
  (bind _asbp_first_person_character (`self.GetPlayer`))
  (bind _asbp_first_person_character_2 (`self.GetPlayer`))
  (bind _asbp_first_person_character_3 (`self.GetPlayer`))
  (bind _jumpoffwall (`self.JumpOffWall`))
  (bind _charactermovement (`Character.CharacterMovement` _asbp_first_person_character_2))
  (bind _maxwalkspeed (`CharacterMovementComponent.MaxWalkSpeed` _charactermovement))
  (bind (_returnvalue_x _returnvalue_y) (`KismetMathLibrary.BreakVector` (* (`SceneComponent.GetForwardVector` (`/Game/Blueprints/BP_FirstPersonCharacter.FirstPersonCamera` _asbp_first_person_character_2)) (+ (/ _maxwalkspeed (`self.WallJumpForwardPlusSpeedingMultiplier`)) (`self.ForwardLaunch`)))))
  (`|ExecutionSequence`
    (:`then_0`
      (if (`/Game/Blueprints/BP_FirstPersonCharacter.Wallrunning?` _asbp_first_person_character)
        (set `local.LaunchDirection` (`KismetMathLibrary.Cross_VectorVector` (* (`/Game/Blueprints/BP_FirstPersonCharacter.WallrunDirection` _asbp_first_person_character) 2.0) (select `/Game/Blueprints/Enums/E_WallrunSide` (`self.WallRunningSide`) :`NewEnumerator0` (`KismetMathLibrary.MakeVector` 0.0 0.0 _jumpoffwall) :`NewEnumerator1` (`KismetMathLibrary.MakeVector` 0.0 0.0 (* _jumpoffwall -1.0)) :!type "Vector Structure")))
        (elif (`NavMovementComponent.IsFalling` (`Character.CharacterMovement` (`self.GetPlayer`)))
          (set `local.LaunchDirection` (+ (* (`Actor.GetActorRightVector` _asbp_first_person_character_3) (`self.RightAxis`)) (* (`Actor.GetActorForwardVector` _asbp_first_person_character_3) (`self.ForwardAxis`)))))))
    (:`then_1`
      (return (* (+ (`local.LaunchDirection`) (`KismetMathLibrary.MakeVector` _returnvalue_x _returnvalue_y (+ (`self.WallJumpHeight`) (/ _maxwalkspeed 1000.0)))) (* (`CharacterMovementComponent.JumpZVelocity` _charactermovement) (`self.WalljumpMultiplier`)))))))

(fn `FindRunDirectionAndSide`
  (params (WallrunNormal :type "Vector Structure"))
  (returns (Direction :type "Vector Structure") (Side :type "/Game/Blueprints/Enums/E_WallrunSide Enum"))
  ;[1 0.3822 0.06732 0.194] Get Side of the WALL
  (bind _output_get (set `self.WallRunningSide` (select `bool` (> (`KismetMathLibrary.DotProduct2D` (`KismetMathLibrary.Conv_VectorToVector2D` WallrunNormal) (`KismetMathLibrary.Conv_VectorToVector2D` (`Actor.GetActorRightVector` (`GameplayStatics.GetPlayerCharacter` 0)))) 0.0) :`false` "NewEnumerator0" :`true` "NewEnumerator1" :!type "/Game/Blueprints/Enums/E_WallrunSide Enum")))
  (return (`KismetMathLibrary.Cross_VectorVector` (`local.WallrunNormal`) (select `/Game/Blueprints/Enums/E_WallrunSide` _output_get :`NewEnumerator0` (0.0 0.0 -1.0) :`NewEnumerator1` (0.0 0.0 1.0) :!type "Vector Structure")) (`self.WallRunningSide`)))

(fn `GetPlayer`
  (returns (`AsBP First Person Character` :type "/Game/Blueprints/BP_FirstPersonCharacter Object Reference"))
  (return (cast `/Game/Blueprints/BP_FirstPersonCharacter` (`GameplayStatics.GetPlayerCharacter` 0) :!pure true)))