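; Player component that throws a katana and lets the character launch toward it as a grapple point.
; Input spawns the katana at the character's launch point as a projectile and flags it thrown.
; While time stop is active, a per-tick camera trace toggles the sword's widget and grapple eligibility.
; LaunchTowardsSword, not called here, flings the character at the sword, halts it and restores a depleted dash; detach and retrieve are empty stubs.
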(event `self.ReceiveBeginPlay`
  (bind _asbp_first_person_character (cast `/Game/Blueprints/BP_FirstPersonCharacter` (`GameplayStatics.GetPlayerCharacter` 0)))
  (bind _output_get (set `self.OwningCharacter` _asbp_first_person_character))
  (set `self.Current Weapon` (`/Game/Blueprints/BP_FirstPersonCharacter.GetCurrentWeapon` _output_get))
  (set `self.E_HasThrown` "NewEnumerator1"))

(event `InputAction|SwordThrow`
  (params (Key :type "Key Structure"))
  (:`Pressed`
    (`self.ThrowSword`)))

(event `self.ReceiveTick`
  (params (DeltaSeconds :type "Float (single-precision)"))
  (`self.CheckIfLookingAtSword`))

(fn `CheckIfHasSword`
  (`/Engine/EditorBlueprintResources/StandardMacros.IsValid` (`self.Current Weapon`)
    (:`Is Valid`
      (return))))

(fn `CheckIfLookingAtSword`
  (locals (Range :type "Float (double-precision)" :default 1000.0))
  (bind _thrownsword (`self.ThrownSword`))
  (bind _widget (`/Game/Blueprints/BP_Katana_Weapon.Widget` (`self.ThrownSword`)))
  (bind _firstpersoncamera (`/Game/Blueprints/BP_FirstPersonCharacter.FirstPersonCamera` (`self.OwningCharacter`)))
  (bind _returnvalue (`SceneComponent.K2_GetComponentLocation` _firstpersoncamera))
  (switch `/Game/Blueprints/Enums/E_TimeStopActive` (`/Game/Blueprints/Components/TimeStopComponent.GetTimeStopActive` (`/Game/Blueprints/BP_FirstPersonCharacter.TimeStopComponent` (`self.OwningCharacter`)))
    (:`NewEnumerator0`
      (`/Engine/EditorBlueprintResources/StandardMacros.IsValid` (`self.ThrownSword`)
        (:`Is Valid`
          (`SceneComponent.SetVisibility` (`/Game/Blueprints/BP_Katana_Weapon.Widget` (`self.ThrownSword`)) false false))))
    (:`NewEnumerator1`
      (bind _outhit (`KismetSystemLibrary.LineTraceSingle` :`Start` _returnvalue :`End` (+ _returnvalue (* (`KismetMathLibrary.GetForwardVector` (`SceneComponent.K2_GetComponentRotation` _firstpersoncamera)) (`local.Range`))) :`TraceChannel` "TraceTypeQuery1" :`DrawDebugType` "ForDuration"))
      (`/Engine/EditorBlueprintResources/StandardMacros.IsValid` _thrownsword
        (:`Is Valid`
          (if (== (`.HitActor` (`GameplayStatics.BreakHitResult` _outhit)) _thrownsword)
            (set `self.E_CanGrapple` "NewEnumerator0")
            (`SceneComponent.SetVisibility` _widget true false)
            (else
              (set `self.E_CanGrapple` "NewEnumerator1")
              (`SceneComponent.SetVisibility` _widget false false))))))))

(fn `DetachSword`)

(fn `GetCanGrapple`
  (returns (E_CanGrapple :type "/Game/Blueprints/Enums/E_CanGrappleTowardsSword Enum"))
  (return (`self.E_CanGrapple`)))

(fn `GetHasThrown`
  (returns (E_HasThrown :type "/Game/Blueprints/Enums/E_HasThrownSword Enum"))
  (return (`self.E_HasThrown`)))

(fn `Launch Towards Sword`
  (bind _owningcharacter (`self.OwningCharacter`))
  (bind _dashleft (`/Game/Blueprints/BP_FirstPersonCharacter.DashLeft` _owningcharacter))
  (`Character.LaunchCharacter` (`self.OwningCharacter`) (* (`KismetMathLibrary.MakeVector` (.x (`KismetMathLibrary.Conv_RotatorToVector` (`KismetMathLibrary.FindLookAtRotation` (`SceneComponent.K2_GetComponentLocation` (`Character.CapsuleComponent` (`self.OwningCharacter`))) (`SceneComponent.K2_GetComponentLocation` (`/Game/Blueprints/BP_Katana_Weapon.DefaultSceneRoot` (`self.ThrownSword`)))))) (.y (`KismetMathLibrary.Conv_RotatorToVector` (`KismetMathLibrary.FindLookAtRotation` (`SceneComponent.K2_GetComponentLocation` (`Character.CapsuleComponent` (`self.OwningCharacter`))) (`SceneComponent.K2_GetComponentLocation` (`/Game/Blueprints/BP_Katana_Weapon.DefaultSceneRoot` (`self.ThrownSword`)))))) (+ (.z (`KismetMathLibrary.Conv_RotatorToVector` (`KismetMathLibrary.FindLookAtRotation` (`SceneComponent.K2_GetComponentLocation` (`Character.CapsuleComponent` (`self.OwningCharacter`))) (`SceneComponent.K2_GetComponentLocation` (`/Game/Blueprints/BP_Katana_Weapon.DefaultSceneRoot` (`self.ThrownSword`)))))) 0.1)) 2800.0) true true)
  (set `MovementComponent.Velocity` (0.0 0.0 0.0) (`/Game/Blueprints/BP_Katana_Weapon.ProjectileMovement` (`self.ThrownSword`)))
  (set `/Game/Blueprints/BP_FirstPersonCharacter.E_CurrentPlayerAction` "NewEnumerator2" _owningcharacter)
  (if (< _dashleft 1)
    (set `/Game/Blueprints/BP_FirstPersonCharacter.DashLeft` (+ _dashleft 1) _owningcharacter)))

(fn `RetrieveSword`)

(fn `ThrowSword`
  (bind _returnvalue (`|SpawnActorFromClass` "/Game/Blueprints/BP_Katana_Weapon.BP_Katana_Weapon_C" (`SceneComponent.K2_GetComponentToWorld` (`/Game/Blueprints/BP_FirstPersonCharacter.LaunchPlace` (`self.OwningCharacter`))) "AlwaysSpawn" "MultiplyWithRoot" null null))
  (set `self.ThrownSword` _returnvalue)
  (`SceneComponent.K2_SetRelativeRotation` (`/Game/Blueprints/BP_Katana_Weapon.StaticMesh` _returnvalue) (struct :`Yaw` 180.0) false false)
  (set `MovementComponent.Velocity` (* (`Actor.GetActorForwardVector` (`self.ThrownSword`)) (`self.SwordThrowSpeed`)) (`/Game/Blueprints/BP_Katana_Weapon.ProjectileMovement` (`self.ThrownSword`)))
  (`PrimitiveComponent.SetCollisionEnabled` (`/Game/Blueprints/BP_Katana_Weapon.Sphere` (`self.ThrownSword`)) "QueryOnly")
  (set `self.E_HasThrown` "NewEnumerator0")
  (`/Game/Blueprints/BP_Katana_Weapon.SetUI` (`self.ThrownSword`)))