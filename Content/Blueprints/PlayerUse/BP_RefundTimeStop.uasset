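; BP_RefundTimeStop is a trigger that refunds the player's time stop cooldown when the first-person character overlaps its Box.
; The overlap calls the character's RefundTSCD and RefundCDTSExtra, and briefly runs its TSCooldown at a much faster play rate before restoring normal speed after a short delay.
; The actor has no logic to disable or destroy itself after use.
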(event `self.Box.OnComponentBeginOverlap`
  (params (OverlappedComponent :type "PrimitiveComponent Object Reference") (OtherActor :type "Actor Object Reference") (OtherComp :type "PrimitiveComponent Object Reference") (OtherBodyIndex :type Integer) (bFromSweep :type Boolean) (SweepResult :type "HitResult Structure (by ref)"))
  (if (== (`GameplayStatics.GetObjectClass` OtherActor) "/Game/Blueprints/BP_FirstPersonCharacter.BP_FirstPersonCharacter_C")
    (bind _asbp_first_person_character (cast `/Game/Blueprints/BP_FirstPersonCharacter` (`GameplayStatics.GetPlayerCharacter` 0)))
    (`/Game/Blueprints/BP_FirstPersonCharacter.RefundTSCD` _asbp_first_person_character)
    (bind _ts_cooldown (`/Game/Blueprints/BP_FirstPersonCharacter.TS_Cooldown` _asbp_first_person_character))
    (`TimelineComponent.SetPlayRate` _ts_cooldown 10.0)
    (`/Game/Blueprints/BP_FirstPersonCharacter.RefundCDTSExtra` _asbp_first_person_character)
    (`KismetSystemLibrary.Delay` 0.5)
    (`TimelineComponent.SetPlayRate` _ts_cooldown 1.0)))

(fn `UserConstructionScript`)