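; BP_UnlockSkill is a one-shot trigger actor that activates a new skill in the player's skill tree.
; When BP_FirstPersonCharacter overlaps its Box, it passes the player's Points to SetNewSkillActive on the SkilltreeComponent's widget.
; It then saves the game through the player's BPCSaving component using that component's save slot, and destroys itself.
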(event `self.Box.OnComponentBeginOverlap`
  (params (OverlappedComponent :type "PrimitiveComponent Object Reference") (OtherActor :type "Actor Object Reference") (OtherComp :type "PrimitiveComponent Object Reference") (OtherBodyIndex :type Integer) (bFromSweep :type Boolean) (SweepResult :type "HitResult Structure (by ref)"))
  (bind _asbp_first_person_character (`self.GetPlayer`))
  (bind _bpc_saving (`/Game/Blueprints/BP_FirstPersonCharacter.BPC_saving` _asbp_first_person_character))
  (if (== (`GameplayStatics.GetObjectClass` OtherActor) "/Game/Blueprints/BP_FirstPersonCharacter.BP_FirstPersonCharacter_C")
    (`/Game/Blueprints/SkillTree/W_SkillClock.SetNewSkillActive` (`/Game/Blueprints/SkillTree/Component/SkilltreeComponent.SkilltreeWidget` (`/Game/Blueprints/BP_FirstPersonCharacter.SkilltreeComponent` _asbp_first_person_character)) (`/Game/Blueprints/BP_FirstPersonCharacter.Points` _asbp_first_person_character))
    (`/Game/Blueprints/SavingAndLoading/BPC_saving.SaveGame` _bpc_saving (`/Game/Blueprints/SavingAndLoading/BPC_saving.Slot Name Save` _bpc_saving))
    (`self.K2_DestroyActor`)))

(fn `GetPlayer`
  (returns (`AsBP First Person Character` :type "/Game/Blueprints/BP_FirstPersonCharacter Object Reference"))
  (return (cast `/Game/Blueprints/BP_FirstPersonCharacter` (`GameplayStatics.GetPlayerCharacter` 0) :!pure true)))

(fn `UserConstructionScript`)