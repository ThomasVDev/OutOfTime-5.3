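; BP_TimeStopExtender is a pickup that renews the player's time stop progress on touch.
; It starts hidden without collision and appears with an active overlap sphere when PlayerUsedTimeStop is called.
; Overlap by BP_FirstPersonCharacter calls RenewTSProgress, then hides and disables the pickup until the next PlayerUsedTimeStop call.
; BeginPlay sets an extremely high CustomTimeDilation on the actor.
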(event `self.ReceiveBeginPlay`
  (set `self.CustomTimeDilation` 100000.0)
  (`SceneComponent.SetVisibility` (`self.DefaultSceneRoot`) false true)
  (`self.SetNotActive`))

(event `PlayerUsedTimeStop`
  (`SceneComponent.SetVisibility` (`self.DefaultSceneRoot`) true true)
  (`PrimitiveComponent.SetCollisionEnabled` (`self.Sphere`) "QueryAndPhysics"))

(event `SetNotActive`
  (`SceneComponent.SetVisibility` (`self.DefaultSceneRoot`) false true)
  (`PrimitiveComponent.SetCollisionEnabled` (`self.Sphere`) "NoCollision"))

(event `self.Sphere.OnComponentBeginOverlap`
  (params (OverlappedComponent :type "PrimitiveComponent Object Reference") (OtherActor :type "Actor Object Reference") (OtherComp :type "PrimitiveComponent Object Reference") (OtherBodyIndex :type Integer) (bFromSweep :type Boolean) (SweepResult :type "HitResult Structure (by ref)"))
  (if (== (`GameplayStatics.GetObjectClass` OtherActor) "/Game/Blueprints/BP_FirstPersonCharacter.BP_FirstPersonCharacter_C")
    (bind _asbp_first_person_character (cast `/Game/Blueprints/BP_FirstPersonCharacter` OtherActor))
    (`/Game/Blueprints/BP_FirstPersonCharacter.RenewTSProgress` _asbp_first_person_character)
    (`self.SetNotActive`)))

(fn `UserConstructionScript`)