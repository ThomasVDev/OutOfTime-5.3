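; BP_SlideRamp is a slide ramp Blueprint that can turn the player's view toward a set point on the ramp.
; On BeginPlay it casts the player character to BP_FirstPersonCharacter and stores it as OwningCharacter.
; RotateCamera plays a timeline that blends the controller's rotation toward the CameraLookAt component's world rotation along the shortest path, lerping from the current rotation on each update.
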(event `self.ReceiveBeginPlay`
  (bind _asbp_first_person_character (cast `/Game/Blueprints/BP_FirstPersonCharacter` (`GameplayStatics.GetPlayerCharacter` 0)))
  (set `self.OwningCharacter` _asbp_first_person_character))

(event `RotateCamera`
  (bind _returnvalue (`GameplayStatics.GetPlayerController` 0))
  (bind (_direction _rotate) (`Timeline|RotateCam` :!via `PlayFromStart`)
    (:`Update`
      (`Controller.SetControlRotation` _returnvalue (`KismetMathLibrary.RLerp` (`Controller.GetControlRotation` _returnvalue) (`SceneComponent.K2_GetComponentRotation` (`self.CameraLookAt`)) _rotate true)))))

(fn `UserConstructionScript`)