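; BP_SwordHook is a hook point that draws in the player's thrown katana.
; It caches the first-person player character on BeginPlay.
; When a katana enters its sphere, it checks the player's SwordThrowComponent and, if the sword has been thrown, calls Magnet on the katana with the hook's root location as the target.
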(event `self.ReceiveBeginPlay`
  (bind _asbp_first_person_character (cast `/Game/Blueprints/BP_FirstPersonCharacter` (`GameplayStatics.GetPlayerCharacter` 0)))
  (set `self.OwningCharacter` _asbp_first_person_character))

(event `self.Sphere.OnComponentBeginOverlap`
  (params (OverlappedComponent :type "PrimitiveComponent Object Reference") (OtherActor :type "Actor Object Reference") (OtherComp :type "PrimitiveComponent Object Reference") (OtherBodyIndex :type Integer) (bFromSweep :type Boolean) (SweepResult :type "HitResult Structure (by ref)"))
  (if (== (`GameplayStatics.GetObjectClass` OtherActor) "/Game/Blueprints/BP_Katana_Weapon.BP_Katana_Weapon_C")
    (bind _asbp_katana_weapon (cast `/Game/Blueprints/BP_Katana_Weapon` OtherActor))
    (switch `/Game/Blueprints/Enums/E_HasThrownSword` (`/Game/Blueprints/Components/SwordThrowComponent.GetHasThrown` (`/Game/Blueprints/BP_FirstPersonCharacter.SwordThrowComponent` (`self.OwningCharacter`)))
      (:`NewEnumerator0`
        (`/Game/Blueprints/BP_Katana_Weapon.Magnet` _asbp_katana_weapon (`SceneComponent.K2_GetComponentLocation` (`self.DefaultSceneRoot`)))))))

(fn `UserConstructionScript`)